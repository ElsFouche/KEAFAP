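; Save game data Blueprint that holds player stats, settings, blood, upgrades and unlocked weapons.
; UpdateSavedStats merges a finished run's stats into per-field single-run bests and running totals; its deprecated blood and level updates are disconnected.
; UpdateSettings stores new settings and broadcasts SettingsUpdated.
; ResetTempData restores default weapon upgrades and the starting weapon unlock, and clears blood and player upgrades.
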(fn UpdateSavedStats
  (params (CurrentRunStats :type F%20Player%20Stats%20Structure%20%28by%20ref%29))
  (bind (_experience _kills _headshotkills _shotsfired _shotshit _headshotshit _blood _timesurvived _timeearned) (Utilities|Struct|BreakF_PlayerStats CurrentRunStats))
  (bind (_experience_2 _kills_2 _headshotkills_2 _shotsfired_2 _shotshit_2 _headshotshit_2 _blood_2 _timesurvived_2 _timeearned_2) (Utilities|Struct|BreakF_PlayerStats CurrentRunStats))
  (bind _statssinglerunbest (Variables|PlayerStats|GetStatsSingleRunBest))
  (bind _statstotals (Variables|PlayerStats|GetStatsTotals))
  (bind (_experience_3 _kills_3 _headshotkills_3 _shotsfired_3 _shotshit_3 _headshotshit_3 _blood_3 _timesurvived_3 _timeearned_3) (Utilities|Struct|BreakF_PlayerStats _statssinglerunbest))
  (bind (_experience_4 _kills_4 _headshotkills_4 _shotsfired_4 _shotshit_4 _headshotshit_4 _blood_4 _timesurvived_4 _timeearned_4) (Utilities|Struct|BreakF_PlayerStats _statstotals))
  ;[0.15 0.15 0.15 0.5] Check for new PBs
  (Utilities|Struct|SetmembersinF_PlayerStats _statssinglerunbest (Math|Integer|Max(Integer) _experience _experience_3) (Math|Integer|Max(Integer) _kills _kills_3) (Math|Integer|Max(Integer) _headshotkills _headshotkills_3) (Class|KismetMathLibrary|MaxInt64 _shotsfired _shotsfired_3) (Class|KismetMathLibrary|MaxInt64 _shotshit _shotshit_3) (Class|KismetMathLibrary|MaxInt64 _headshotshit _headshotshit_3) (Math|Integer|Max(Integer) _blood _blood_3) (Class|KismetMathLibrary|MaxInt64 _timesurvived _timesurvived_3) (Class|KismetMathLibrary|MaxInt64 _timeearned _timeearned_3))
  (Utilities|Struct|SetmembersinF_PlayerStats _statstotals (+ _experience_4 _experience_2) (+ _kills_4 _kills_2) (+ _headshotkills_4 _headshotkills_2) (+ _shotsfired_4 _shotsfired_2) (+ _shotshit_4 _shotshit_2) (+ _headshotshit_4 _headshotshit_2) (+ _blood_4 _blood_2) (+ _timesurvived_4 _timesurvived_2) (+ _timeearned_4 _timeearned_2)))

(fn UpdateSettings
  (params (NewSettings :type F%20Settings%20Structure))
  (bind _output_get (Variables|Settings|SetSettings NewSettings))
  (Default|CallSettingsUpdated _output_get))

(fn ResetTempData
  (Variables|Progression|SetWeaponUpgrades (Utilities|Map|MakeMap "NewEnumerator1" 0 "NewEnumerator2" 0 "NewEnumerator4" 0 "NewEnumerator5" 0 "NewEnumerator6" 0 "NewEnumerator7" 0))
  (Variables|Progression|SetPlayerBlood 0)
  (Variables|Progression|SetUnlockedWeapons (Utilities|Array|MakeArray "NewEnumerator1"))
  (Utilities|Array|Clear (Variables|Progression|GetPlayerUpgrades))
  (return))