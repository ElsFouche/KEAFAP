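; BP_FleshCubeExplosion is a short-lived flesh cube explosion actor built around a Geometry Collection.
; On BeginPlay it launches the collection upward and along the player character's forward vector with an impulse.
; After a brief delay it spawns the NS_FleshCube Niagara effect at its location, then destroys itself a few seconds later.
; A note in the graph marks the BeginPlay trigger to be changed to an on-killed event.
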(event EventBeginPlay
  (bind _returnvalue (Game|GetPlayerCharacter 0))
  (bind _returnvalue_2 (Transformation|GetActorForwardVector _returnvalue))
  (bind (_x _y) (Math|Vector|BreakVector _returnvalue_2))
  ;[0.15 0.15 0.15 0.5] Change to on killed
  (Physics|AddImpulse (Variables|Default|GetGeometryCollectionComponent) (Math|Vector|MakeVector (* _x 2e+04) (* _y 2e+04) 3.6e+04) "None" false)
  (Utilities|FlowControl|Delay 0.2)
  (Niagara|SpawnSystematLocation "/Game/FleshCube/NS_FleshCube.NS_FleshCube" (Transformation|GetActorLocation) "0, 0, 0" "2.000000,2.000000,2.000000")
  (Utilities|FlowControl|Delay 5.0)
  (Actor|DestroyActor))

(fn ConstructionScript)