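; BP_DebugActor is a debug helper that skips warmup and can repeatedly damage the player pawn.
; On BeginPlay it registers as a game state listener, unregisters on destruction, and a tick later messages the first player controller with SkipWarmup.
; When enabled, Tick runs a self-repeating Delay loop that applies configurable damage at a set interval.
; A timer-based version with a fixed-damage DamageLoop event is left disconnected.
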(event Custom|OnDestroyedEvent
  (params (DestroyedActor :type Actor%20Object%20Reference))
  (Class|BPIGameState|UnregisterListener(Message) (Game|GetGameState) DestroyedActor))

(event Custom|DamageLoop
  (Game|Damage|ApplyDamage (Game|Player|GetPlayerPawn 0) 5.0 0 0))

(event EventBeginPlay
  (Class|BPIGameState|RegisterNewListener(Message) (Game|GetGameState) self)
  (Game|BindEventtoOnDestroyed (EventDispatchers|CreateEvent :!event Custom|OnDestroyedEvent))
  (Utilities|FlowControl|DelayUntilNextTick)
  (Class|BPIDebug|WarmupSkip(Message) (Game|GetPlayerController 0) (Variables|Debug|GetSkipWarmup)))

(event EventTick
  (params (DeltaSeconds :type Float%20%28single-precision%29))
  (if (Variables|Debug|GetEnableDamageLoop) :!label _label
    (Utilities|FlowControl|Delay (Variables|Debug|GetDamageLoopInterval))
    (Game|Damage|ApplyDamage (Game|Player|GetPlayerPawn 0) (Variables|Debug|GetDamageLoopDamage) 0 0)
    (goto _label)))

(fn ConstructionScript)