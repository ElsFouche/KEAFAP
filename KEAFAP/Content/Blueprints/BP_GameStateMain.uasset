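; Main game state that runs a timed wave, from animated countdown intro to game over.
; Chained timer-widget animation callbacks play the intro, then start a looping countdown, enable autosave and notify registered listeners that warmup is done.
; The clock ticks in integer milliseconds and accepts time adjustments.
; Timeout or player death stops it, shows the death screen, disables input and autosave, saves and pauses the game.
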(event Custom|Timer
  ;[0.15 0.15 0.15 0.5] Countdown timer logic
  (bind _output_get (Variables|CountdownTimer|SetRemainingTime (- (Variables|CountdownTimer|GetRemainingTime) (Math|Float|Round (* (Math|Float|Max(Float) (Utilities|Time|GetWorldDeltaSeconds) (Variables|CountdownTimer|GetTickDownRate)) 1e+03)))))
  (if (> _output_get 0)
    (Default|TimerUpdate (Variables|Components|GetTimerWidget) _output_get)
    (else
      ;[0.15 0.15 0.15 0.5] Player has run out of time in the level.
      (CallFunction|GameOver))))

(event Custom|TextAnimComplete
  (params (CompleteAnim :type E_FontAnims%20Enum :default "NewEnumerator0"))
  (bind _timerwidget (Variables|Components|GetTimerWidget))
  ;[0.15 0.15 0.15 0.5] Startup animations. This is the wrong way to go about it - I didn't know about widget's having their own built-in animation timelines.
  ;;[0.15 0.15 0.15 0.5] It's messy, but this allows us to change up each number's color, size, opacity, easing function, etc.
  (switch Utilities|FlowControl|Switch|SwitchonE_FontAnims CompleteAnim
    (:NewEnumerator0
      (Default|Play0to1Timeline _timerwidget "NewEnumerator1" 0.0))
    (:NewEnumerator1
      (Default|Play0to1Timeline _timerwidget "NewEnumerator2" 0.0))
    (:NewEnumerator2
      (Default|Play0to1Timeline _timerwidget "NewEnumerator3" 0.0))
    (:NewEnumerator3
      (Default|Play0to1Timeline _timerwidget "NewEnumerator4" 0.5)
      ;;[0.15 0.15 0.15 0.5] Start level
      ;;;[0.15 0.15 0.15 0.5] Start level timer
      (Variables|CountdownTimer|SetRemainingTime (CallFunction|FTimetoInt (Variables|CountdownTimer|GetWaveTimeMax)))
      (bind _returnvalue (Utilities|Time|SetTimerbyEvent (EventDispatchers|CreateEvent :!event Custom|Timer) (Variables|CountdownTimer|GetTickDownRate) true true))
      (Variables|CountdownTimer|SetCountdownTimer _returnvalue)
      ;;;[0.15 0.15 0.15 0.5] Enable autosaving
      (Class|BPISaveGame|SetAutosaving(Message) (Game|GetGameInstance) true)
      ;;;[0.15 0.15 0.15 0.5] Notify disabled gameplay objects to enable.
      (for _array_element (Variables|Gameplay|Events|GetSubscribers)
        (Class|BPIGameState|WarmupDone(Message) _array_element)))))

(event Custom|GameOver
  (bind _returnvalue (Game|GetGameInstance))
  (bind _returnvalue_2 (Game|GetPlayerController 0))
  (bind _deathwidget (Variables|Components|GetDeathWidget))
  ;[0.15 0.15 0.15 0.5] Gameover from player running out of health or time
  (Utilities|Time|ClearandInvalidateTimerbyHandle (Variables|CountdownTimer|GetCountdownTimer))
  (Default|TimerUpdate (Variables|Components|GetTimerWidget))
  ;;[0.15 0.15 0.15 0.5] Disable player input and bring up the game over screen
  (Input|DisableInput (Game|Player|GetPlayerPawn 0) (Game|GetPlayerController 0))
  (Widget|SetVisibility _deathwidget "Visible")
  (Input|SetInputModeGameandUI _returnvalue_2 _deathwidget "LockInFullscreen" false true)
  (Variables|/Script/Engine.PlayerController|SetbShowMouseCursor _returnvalue_2 true)
  ;;[0.15 0.15 0.15 0.5] Disable autosave, update stats, & save game to slot.
  (Class|BPISaveGame|SetAutosaving(Message) _returnvalue false)
  (Class|BPISaveGame|SaveGame(Message) _returnvalue false)
  ;;[0.15 0.15 0.15 0.5] Set the game paused to prevent enemy movement.
  (Game|SetGamePaused true))

(event EventBeginPlay
  ;[0.15 0.15 0.15 0.5] Timer Widget
  ;;[0.15 0.15 0.15 0.5] Initialize the timer widget.
  (bind _returnvalue (UserInterface|CreateWidget "/Game/UI/WBP_Timer.WBP_Timer_C" (Game|GetPlayerController 0)))
  (bind _output_get (Variables|Components|SetTimerWidget _returnvalue))
  (UserInterface|Viewport|AddtoViewport _output_get 0)
  (Default|SetCountdownTime _output_get (Variables|CountdownTimer|GetWaveTimeMax))
  ;;[0.15 0.15 0.15 0.5] The pre-loop delay allows for the timer text to pause in the center of the screen before it moves to the top
  (Default|Play0to1Timeline _output_get "NewEnumerator0" (Variables|CountdownTimer|GetTimerMoveDelay))
  ;[0.15 0.15 0.15 0.5] Death widget - this is handled here because I'm considering "game over" to be a game state rather than player state.
  (bind _returnvalue_2 (UserInterface|CreateWidget "/Game/UI/WBP_DeathScreen.WBP_DeathScreen_C" (Game|GetPlayerController 0)))
  (bind _output_get_2 (Variables|Components|SetDeathWidget _returnvalue_2))
  (UserInterface|Viewport|AddtoViewport _output_get_2 10))

(event EventRegisterNewListener
  (params (Actor :type Actor%20Object%20Reference))
  ;[0.15 0.15 0.15 0.5] What are these for, Els?
  (Utilities|Array|AddUnique (Variables|Gameplay|Events|GetSubscribers) Actor))

(event EventUnregisterListener
  (params (Actor :type Actor%20Object%20Reference))
  ;[0.15 0.15 0.15 0.5] What are these for, Els?
  (Utilities|Array|RemoveItem (Variables|Gameplay|Events|GetSubscribers) Actor))

(event EventPlayerDeath
  (bind _returnvalue (Game|GetGameInstance))
  (bind _returnvalue_2 (Game|GetPlayerController 0))
  (bind _deathwidget (Variables|Components|GetDeathWidget))
  ;[0.15 0.15 0.15 0.5] Gameover from player running out of health or time
  (Utilities|Time|ClearandInvalidateTimerbyHandle (Variables|CountdownTimer|GetCountdownTimer))
  (Default|TimerUpdate (Variables|Components|GetTimerWidget))
  ;;[0.15 0.15 0.15 0.5] Disable player input and bring up the game over screen
  (Input|DisableInput (Game|Player|GetPlayerPawn 0) (Game|GetPlayerController 0))
  (Widget|SetVisibility _deathwidget "Visible")
  (Input|SetInputModeGameandUI _returnvalue_2 _deathwidget "LockInFullscreen" false true)
  (Variables|/Script/Engine.PlayerController|SetbShowMouseCursor _returnvalue_2 true)
  ;;[0.15 0.15 0.15 0.5] Disable autosave, update stats, & save game to slot.
  (Class|BPISaveGame|SetAutosaving(Message) _returnvalue false)
  (Class|BPISaveGame|SaveGame(Message) _returnvalue false)
  ;;[0.15 0.15 0.15 0.5] Set the game paused to prevent enemy movement.
  (Game|SetGamePaused true))

(event EventAddTimetoClock
  (params (ExtraTime :type Integer))
  (bind _output_get (Variables|CountdownTimer|SetRemainingTime (Math|Integer|Max(Integer) (+ (Variables|CountdownTimer|GetRemainingTime) ExtraTime))))
  (Default|TimerUpdate (Variables|Components|GetTimerWidget) _output_get))

(fn ConstructionScript)

(fn GetRemainingTime
  (return (Variables|CountdownTimer|GetRemainingTime)))