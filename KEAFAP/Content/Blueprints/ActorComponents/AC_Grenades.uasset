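; Actor component that spawns and throws a physics grenade of a requested type on behalf of an instigator.
; ThrowGrenade maps the type to a BP_GrenadeBase class; only Fire and Ice have their own, while Electric, Nuke and Gravity reuse the Ice grenade.
; It launches the grenade with a mass-independent impulse along the throw vector, then adds an off-center impulse along the instigator's forward to induce tumble.
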(event Custom|ThrowGrenade
  (params (GrenadeType :type E_GrenadeTypes%20Enum :default "NewEnumerator0") (ThrowStartLocation :type Vector) (ThrowForwardVector :type Vector) (ThrowStrength :type Float%20%28double-precision%29) (Instigator :type Pawn%20Object%20Reference))
  (bind _rootcomponent (Variables|/Script/Engine.Actor|GetRootComponent Instigator))
  (bind _returnvalue (Math|Vector|GetForwardVector _rootcomponent))
  (bind _returnvalue_2 (Game|SpawnActorfromClass (Utilities|Select :Index GrenadeType :NewEnumerator0 "/Game/Blueprints/Grenades/BP_GrenadeBase.BP_GrenadeBase_C" :NewEnumerator1 "/Game/Blueprints/Grenades/BP_IceGrenade.BP_IceGrenade_C" :NewEnumerator3 "/Game/Blueprints/Grenades/BP_IceGrenade.BP_IceGrenade_C" :NewEnumerator2 "/Game/Blueprints/Grenades/BP_IceGrenade.BP_IceGrenade_C" :NewEnumerator4 "/Game/Blueprints/Grenades/BP_IceGrenade.BP_IceGrenade_C" :NewEnumerator5 "/Game/Blueprints/Grenades/BP_FireGrenade.BP_FireGrenade_C") (Math|Transform|MakeTransform ThrowStartLocation "0, 0, 0" "1.000000,1.000000,1.000000") "AlwaysSpawn" "MultiplyWithRoot" 0 Instigator))
  (bind _asbp_grenade_base (Utilities|Casting|CastToBP_GrenadeBase _returnvalue_2))
  (Physics|AddImpulse (Variables|/Game/Blueprints/Grenades/BP_GrenadeBase.BP_GrenadeBase_C|GetGrenade _asbp_grenade_base) (* ThrowForwardVector ThrowStrength) "None" true)
  (Physics|AddImpulseatLocation (Variables|/Game/Blueprints/Grenades/BP_GrenadeBase.BP_GrenadeBase_C|GetGrenade _asbp_grenade_base) (* _returnvalue 1e+03) (+ (Transformation|GetWorldLocation (Variables|/Game/Blueprints/Grenades/BP_GrenadeBase.BP_GrenadeBase_C|GetGrenade _asbp_grenade_base)) (* (Math|Vector|GetUpVector (Variables|/Game/Blueprints/Grenades/BP_GrenadeBase.BP_GrenadeBase_C|GetGrenade _asbp_grenade_base)) 2e+01) (* _returnvalue -5.0)) "None"))