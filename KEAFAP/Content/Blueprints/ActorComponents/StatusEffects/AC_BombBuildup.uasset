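; Status effect component that stacks bomb buildup on its owner and makes it explode once the buildup passes a threshold.
; Re-applying the effect adds to Param; crossing the threshold fires a one-time radial damage with falloff at the owner, credited to player 0, then ends the effect.
; Otherwise, each expiry decrements Param and renews a short Duration until the buildup runs out.
; Explosion VFX is only a debug print.
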(event EventBeginPlay
  (|CallParentFunction) ; This node is disabled and will not be called.\nDrag off pins to build functionality.
)

(event EventEndEffect
  (bind _result (Math|Float|DecrementFloat (Variables|Default|GetParam))
    (:%20%20
      (if (> _result 0.0)
        (Variables|Default|SetDuration 1.0)
        (else
          (|CallParentFunction))))))

(event EventOnSameEffectAdded
  (params (ParamChange :type Float%20%28double-precision%29))
  (bind _returnvalue (Components|GetOwner))
  (bind _returnvalue_2 (Math|Float|MakeLiteralFloat 1e+02))
  (bind _returnvalue_3 (Math|Float|MakeLiteralFloat 2e+02))
  (bind _output_get (Variables|Default|SetParam (+ ParamChange (Variables|Default|GetParam))))
  (if (> _output_get 15.0)
    (Utilities|FlowControl|DoOnce false
      (:Completed
        ;[0.15 0.15 0.15 0.5] Explosion logic
        (Class|GameplayStatics|ApplyRadialDamagewithFalloff _returnvalue_3 (* _returnvalue_3 0.1) (Transformation|GetActorLocation _returnvalue) (* _returnvalue_2 0.5) (* _returnvalue_2 1.5) 2.0 0 0 _returnvalue (Game|GetPlayerController 0) "ECC_WorldStatic")
        ;;[0.15 0.15 0.15 0.5] VFX
        (Development|PrintString "Boom")
        (Variables|Default|SetParam 0.0)
        (Variables|Default|SetDuration 0.0)
        (CallFunction|EndEffect)))))

(event EventTick
  (params (DeltaSeconds :type Float%20%28single-precision%29))
  (|CallParentFunction DeltaSeconds))