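; Base actor component for timed status effects, which lives on the affected actor until its duration runs out.
; On BeginPlay it looks for another component of its own class on the owner; if one exists, it adds its Duration to the first found and destroys itself, so repeat applications extend the effect.
; Tick counts Duration down and calls EndEffect at zero, which destroys the component.
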(event Custom|OwnerAlreadyHasThis
  (params (Original%20Component :type AC%20Status%20Effect%20Base%20Object%20Reference))
  (Variables|AC_StatusEffectBase_C|SetDuration Original%20Component (+ (Variables|AC_StatusEffectBase_C|GetDuration Original%20Component) (Variables|Default|GetDuration)))
  (Components|DestroyComponent))

(event Custom|EndEffect
  (Components|DestroyComponent))

(event EventBeginPlay
  (bind _returnvalue (Components|GetOwner))
  (bind _self self)
  (bind _returnvalue_2 (Utilities|GetClass _self))
  (bind _returnvalue_3 (Actor|GetComponentsByClass _returnvalue _returnvalue_2))
  (if (> (Utilities|Array|Length _returnvalue_3) 1)
    (CallFunction|OwnerAlreadyHasThis (Utilities|Array|Get(acopy) _returnvalue_3))))

(event EventTick
  (params (DeltaSeconds :type Float%20%28single-precision%29))
  (bind _output_get (Variables|Default|SetDuration (- (Variables|Default|GetDuration) DeltaSeconds)))
  (if (<= _output_get 0.0)
    (CallFunction|EndEffect)))