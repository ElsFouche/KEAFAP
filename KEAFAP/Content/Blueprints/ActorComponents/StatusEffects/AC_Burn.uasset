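; AC_Burn is a status effect actor component that deals damage over time to its owner.
; On BeginPlay it starts a looping one-second timer, unless one is already valid, that fires Burn with Param as the damage.
; BP_Player owners take it through ApplyDamage, while other owners receive it through the ApplyGenericDamageMessage call.
; EndEffect clears and invalidates the timer before running the parent's end logic.
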(event Custom|Burn
  (bind _returnvalue (Components|GetOwner))
  (bind _param (Variables|Default|GetParam))
  (Class|KismetSystemLibrary|IsObjectOfSoftClass _returnvalue "/Game/Blueprints/FirstPerson/BP_Player.BP_Player_C"
    (:True
      (Game|Damage|ApplyDamage _returnvalue _param 0 0))
    (:False
      (Class|BPITakeDamage|ApplyGenericDamage(Message) _returnvalue _param))))

(event EventBeginPlay
  (|CallParentFunction)
  (if (not (Utilities|Time|IsValidTimerHandle (Variables|Default|GetBurnTimer)))
    (bind _returnvalue (Utilities|Time|SetTimerbyEvent (delegate Custom|Burn) 1.0 true))
    (Variables|Default|SetBurnTimer _returnvalue)))

(event EventEndEffect
  (Utilities|Time|ClearandInvalidateTimerbyHandle (Variables|Default|GetBurnTimer))
  (|CallParentFunction))