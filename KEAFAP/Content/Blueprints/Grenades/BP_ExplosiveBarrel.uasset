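; Explosive barrel that detonates the first time it takes any damage, guarded by a DoOnce.
; Detonation spawns a pooled Niagara explosion with a set force parameter and a fire hazard actor, then hides the barrel mesh and disables its collision.
; A separate Respawn event restores the mesh and collision after a delay, but nothing here calls it or resets the DoOnce.
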(event Custom|Respawn
  (bind _barrel1 (Variables|Default|GetBarrel1))
  (Utilities|FlowControl|Delay 25.0)
  (Rendering|SetVisibility _barrel1 true false)
  (Collision|SetCollisionEnabled _barrel1 "QueryAndPhysics"))

(event Game|Damage|EventAnyDamage
  (params (Damage :type Float%20%28single-precision%29) (DamageType :type Damage%20Type%20Object%20Reference) (InstigatedBy :type Controller%20Object%20Reference) (DamageCauser :type Actor%20Object%20Reference))
  (bind _defaultsceneroot (Variables|Default|GetDefaultSceneRoot))
  (bind _barrel1 (Variables|Default|GetBarrel1))
  (bind _returnvalue (Transformation|GetWorldLocation _defaultsceneroot))
  (Utilities|FlowControl|DoOnce false
    (:Completed
      (bind _returnvalue_2 (Niagara|SpawnSystematLocation "/Game/Particles/NS_Explosion.NS_Explosion" _returnvalue (Transformation|GetWorldRotation _defaultsceneroot) "1.000000,1.000000,1.000000" true true "AutoRelease"))
      (Niagara|SetNiagaraVariable(Float) _returnvalue_2 "ExplosionForce" 1e+02)
      (Game|SpawnActorfromClass "/Game/Blueprints/Grenades/BP_HazardFire.BP_HazardFire_C" (Math|Transform|MakeTransform _returnvalue "0, 0, 0" "1.000000,1.000000,1.000000") "Undefined" "MultiplyWithRoot" 0 0)
      (Rendering|SetVisibility _barrel1 false false)
      (Collision|SetCollisionEnabled _barrel1 "NoCollision"))))

(fn ConstructionScript)