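; Base grenade Blueprint that detonates after a fuse delay triggered by a blocking hit, leaving the explosion effect to child classes.
; After the fuse, a DoOnce-guarded multi-sphere trace at the grenade's location gathers objects within the blast radius, ignoring player 0's pawn and drawing debug shapes.
; Hits are reduced to unique actors, each passed to the empty OnExplosion event for children to implement, then the grenade destroys itself.
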(event OnComponentHit(Grenade)
  (params (HitComponent :type Primitive%20Component%20Object%20Reference) (OtherActor :type Actor%20Object%20Reference) (OtherComp :type Primitive%20Component%20Object%20Reference) (NormalImpulse :type Vector :default "0, 0, 0") (Hit :type Hit%20Result%20Structure%20%28by%20ref%29))
  (bind _grenade (Variables|Default|GetGrenade))
  (bind _returnvalue (Transformation|GetWorldLocation _grenade))
  (if (.bBlockingHit (Collision|BreakHitResult Hit))
    (Utilities|FlowControl|Delay (Variables|Grenade|GetFuseTime))
    (Utilities|FlowControl|DoOnce false
      (:Completed
        ;[0.15 0.15 0.15 0.5] Explosion Logic
        (bind _outhits (Collision|MultiSphereTraceForObjects _returnvalue _returnvalue (Variables|Grenade|GetBlastRadius) (Utilities|Array|MakeArray "ObjectTypeQuery2" "ObjectTypeQuery3" "ObjectTypeQuery4" "ObjectTypeQuery6") false (Utilities|Array|MakeArray (Game|Player|GetPlayerPawn 0)) "ForDuration"))
        (bind _uniqueactors (CallFunction|UniqueActorsHit _outhits))
        (for _array_element _uniqueactors
          (CallFunction|OnExplosion _array_element))
        (Actor|DestroyActor)))))

(event Custom|OnExplosion
  (params (HitActor :type Actor%20Object%20Reference))
  ;[0.15 0.15 0.15 0.5] Implemented in children
)

(fn ConstructionScript)