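; BP_HazardFire is a fire hazard area, filed with the grenades, that burns and damages actors inside it.
; It overrides its parent's area events: actors in the area receive AC_Burn and Damage, applied either directly or via a message, depending on a class check.
; Leaving applies a short timed burn carrying Damage, using a direct AddACBurn call for BP_Player and a status-effect message for other actors.
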(event EventBeginPlay
  (|CallParentFunction))

(event EventOnLeaveArea
  (params (ExitingActor :type Actor%20Object%20Reference))
  (Class|KismetSystemLibrary|IsObjectOfSoftClass ExitingActor "/Game/Blueprints/FirstPerson/BP_Player.BP_Player_C"
    (:True
      (Game|AddComponentbyClass ExitingActor "/Game/Blueprints/ActorComponents/StatusEffects/AC_Burn.AC_Burn_C" 3.1 (Variables|Hazard|GetDamage) 0 0))
    (:False
      (Class|BPIEnemyAI|ApplyStatusEffect(Message) ExitingActor "/Game/Blueprints/ActorComponents/StatusEffects/AC_Burn.AC_Burn_C" 3.1 (Variables|Hazard|GetDamage)))))

(event EventInAreaEffects
  (params (ActorInRegion :type Actor%20Object%20Reference))
  (bind _damage (Variables|Hazard|GetDamage))
  (Utilities|IsValid ActorInRegion
    (:Is%20Valid
      (Class|BPIEnemyAI|ApplyStatusEffect(Message) ActorInRegion "/Game/Blueprints/ActorComponents/StatusEffects/AC_Burn.AC_Burn_C" 0.0 0.0)
      (Class|KismetSystemLibrary|IsObjectOfSoftClass ActorInRegion "/Game/Blueprints/FirstPerson/BP_Player.BP_Player_C"
        (:True
          (Game|Damage|ApplyDamage ActorInRegion _damage 0 0))
        (:False
          (Class|BPITakeDamage|ApplyGenericDamage(Message) ActorInRegion _damage))))))

(fn ConstructionScript
  (|CallParentFunction))