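; Rocket projectile that launches with a slight upward kick, then eases toward max speed along its initial heading after a short delay.
; An armed blocking hit on anything but the player sphere-traces to launch nearby characters away, applies falloff radial damage sparing the player, and destroys the rocket.
; Other hits drop it into physics with full gravity and arm the warhead after a random delay.
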(event OnComponentHit(Collision)
  (params (HitComponent :type Primitive%20Component%20Object%20Reference) (OtherActor :type Actor%20Object%20Reference) (OtherComp :type Primitive%20Component%20Object%20Reference) (NormalImpulse :type Vector :default "0, 0, 0") (Hit :type Hit%20Result%20Structure%20%28by%20ref%29))
  (bind _blastradius (Variables|Rocket|GetBlastRadius))
  (bind _rocket (Variables|Default|GetRocket))
  (bind _damage (Variables|Rocket|GetDamage))
  (bind _returnvalue (Transformation|GetWorldLocation _rocket))
  (if (and (.bBlockingHit (Collision|BreakHitResult Hit)) (Variables|Default|GetbWarheadActive))
    (Class|KismetSystemLibrary|IsObjectOfSoftClass OtherActor "/Game/Blueprints/FirstPerson/BP_Player.BP_Player_C"
      (:False
        (Utilities|FlowControl|DoOnce false
          (:Completed
            ;[0.15 0.15 0.15 0.5] Explosion Logic
            (bind _outhits (Collision|MultiSphereTraceForObjects _returnvalue _returnvalue (Variables|Rocket|GetBlastRadius) (Utilities|Array|MakeArray "ObjectTypeQuery2" "ObjectTypeQuery3" "ObjectTypeQuery4" "ObjectTypeQuery6") false 0 "ForDuration"))
            (bind _uniqueactors (CallFunction|UniqueActorsHit _outhits))
            (for _array_element _uniqueactors
              (CallFunction|OnExplosionEffects _array_element))
            ;[0.15 0.15 0.15 0.5] Apply damage and destroy actor
            (Class|GameplayStatics|ApplyRadialDamagewithFalloff _damage (* _damage 0.1) (Transformation|GetWorldLocation (Variables|Default|GetRocket)) (* _blastradius 0.5) (* _blastradius 1.5) 2.0 0 (Utilities|Array|MakeArray (Game|Player|GetPlayerPawn 0)) self (Game|GetPlayerController 0) "ECC_Visibility")
            (Actor|DestroyActor)))))
    (else
      (Variables|Default|SetbPrematureImpact true)
      (Physics|SetSimulatePhysics (Variables|Default|GetCollision) true)
      (Variables|/Script/Engine.ProjectileMovementComponent|SetProjectileGravityScale (Variables|Default|GetProjectileMovement) 1.0)
      (Utilities|FlowControl|Delay (Math|Random|RandomFloatinRange 0.5 2.0))
      (Variables|Default|SetbWarheadActive true))))

(event Custom|OnExplosionEffects
  (params (HitActor :type Actor%20Object%20Reference))
  (bind _ascharacter (Utilities|Casting|CastToCharacter HitActor))
  (Character|LaunchCharacter _ascharacter (* (Math|Vector|Normalize (- (Transformation|GetActorLocation HitActor) (Transformation|GetWorldLocation (Variables|Default|GetRocket)))) (Variables|Rocket|GetLaunchPower)) false false))

(event EventBeginPlay
  (bind _returnvalue (Transformation|GetActorForwardVector))
  (Variables|Default|SetStartForward _returnvalue)
  (Variables|/Script/Engine.MovementComponent|SetVelocity (Variables|Default|GetProjectileMovement) (+ (* _returnvalue (Variables|Rocket|GetStartSpeed)) (* (Transformation|GetActorUpVector) 1e+02)))
  (Utilities|FlowControl|Delay 0.3)
  (Variables|/Script/Engine.ProjectileMovementComponent|SetProjectileGravityScale (Variables|Default|GetProjectileMovement) 0.02)
  (bind _alpha (Utilities|AsyncTick 0.2)
    (:Tick
      (Variables|/Script/Engine.MovementComponent|SetVelocity (Variables|Default|GetProjectileMovement) (Math|Interpolation|Ease "CircularIn" _alpha (* (Variables|Rocket|GetStartSpeed) (Transformation|GetActorForwardVector)) (* (Variables|Default|GetStartForward) (Variables|Rocket|GetMaxSpeed)))))))

(fn ConstructionScript)