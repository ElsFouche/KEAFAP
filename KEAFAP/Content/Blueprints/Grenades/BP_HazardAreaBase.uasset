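; Base hazard area for grenades: a timed-lifespan volume, scaled from Radius and Height, that applies effects to actors inside it.
; Overlap events maintain the ActorsInArea list, and the first overlap starts a looping timer that lasts until the area is destroyed.
; The timer drives per-actor InAreaEffects and prunes invalid entries.
; Children implement InAreaEffects and OnLeaveArea, the latter called when an actor exits.
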(event OnComponentBeginOverlap(HazardArea)
  (params (OverlappedComponent :type Primitive%20Component%20Object%20Reference) (OtherActor :type Actor%20Object%20Reference) (OtherComp :type Primitive%20Component%20Object%20Reference) (OtherBodyIndex :type Integer) (bFromSweep :type Boolean) (SweepResult :type Hit%20Result%20Structure%20%28by%20ref%29))
  (Utilities|Array|AddUnique (Variables|Hazard|GetActorsInArea) OtherActor)
  (if (not (Utilities|Time|IsValidTimerHandle (Variables|Hazard|GetEffectsTimer)))
    (bind _returnvalue (Utilities|Time|SetTimerbyEvent (EventDispatchers|CreateEvent :!event Custom|ForEachInArea) (Variables|Hazard|GetEffectLoopTime) true true))
    (Variables|Hazard|SetEffectsTimer _returnvalue)))

(event OnComponentEndOverlap(HazardArea)
  (params (OverlappedComponent :type Primitive%20Component%20Object%20Reference) (OtherActor :type Actor%20Object%20Reference) (OtherComp :type Primitive%20Component%20Object%20Reference) (OtherBodyIndex :type Integer))
  (CallFunction|OnLeaveArea OtherActor)
  (Utilities|Array|RemoveItem (Variables|Hazard|GetActorsInArea) OtherActor))

(event Custom|SetArea
  (params (Radius :type Float%20%28double-precision%29) (Height :type Float%20%28double-precision%29))
  (bind _returnvalue (/ Radius 5e+01))
  (Transformation|SetRelativeScale3D (Variables|Default|GetHazardPivot) (Math|Vector|MakeVector _returnvalue _returnvalue (/ Height 1e+02))))

(event Custom|InAreaEffects
  (params (ActorInRegion :type Actor%20Object%20Reference))
  ;[0.15 0.15 0.15 0.5] Implemented in children
)

(event Custom|ForEachInArea
  (bind _arrayelement (Utilities|ForEachLoopReal (Variables|Hazard|GetActorsInArea) :!label _label)
    (:LoopBody
      (Utilities|IsValid _arrayelement
        (:Is%20Valid
          (CallFunction|InAreaEffects _arrayelement)
          (goto _label Continue))
        (:Is%20Not%20Valid
          (Utilities|Array|RemoveItem (Variables|Hazard|GetActorsInArea) _arrayelement)
          (goto _label Continue))))))

(event Custom|OnDestroyed_Event
  (params (DestroyedActor :type Actor%20Object%20Reference))
  (Utilities|Time|ClearandInvalidateTimerbyHandle (Variables|Hazard|GetEffectsTimer)))

(event Custom|OnLeaveArea
  (params (ExitingActor :type Actor%20Object%20Reference))
  ;[0.15 0.15 0.15 0.5] Implemented in children
)

(event EventBeginPlay
  (Game|AssignOnDestroyed (delegate Custom|OnDestroyed_Event))
  (CallFunction|SetArea (Variables|Hazard|GetRadius) (Variables|Hazard|GetHeight))
  (Actor|SetLifeSpan (Variables|Hazard|GetIn%20Lifespan)))

(fn ConstructionScript)