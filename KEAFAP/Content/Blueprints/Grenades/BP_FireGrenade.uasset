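; BP_FireGrenade is a grenade Blueprint that leaves a fire hazard on the surface where it explodes.
; Both explosion events, with effects or with no target, feed one DoOnce, so the response fires only once.
; It plays a 2D fire sound, then line traces vertically from above the grenade to far below it.
; A blocking hit spawns BP_HazardFire at the impact point.
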(event EventOnExplosionNoTarget
  (bind _grenade (Variables|Default|GetGrenade))
  (bind _returnvalue (Transformation|GetWorldLocation _grenade))
  (Utilities|FlowControl|DoOnce false
    (:Completed
      (Class|GameplayStatics|PrimeSound "/Game/ModelTextureArtTest/IceGrenade/FireGrenade_SFX_Cue.FireGrenade_SFX_Cue")
      (Audio|PlaySound2D "/Game/ModelTextureArtTest/IceGrenade/FireGrenade_SFX_Cue.FireGrenade_SFX_Cue" 1.0 1.0 0.0 0 0)
      (bind _outhit (Collision|LineTraceByChannel (+ _returnvalue "0.000000,0.000000,1000.000000") (- _returnvalue "0.000000,0.000000,20000.000000") "TraceTypeQuery1" true 0 "None"))
      (if (.bBlockingHit (Collision|BreakHitResult _outhit))
        (Game|SpawnActorfromClass "/Game/Blueprints/Grenades/BP_HazardFire.BP_HazardFire_C" (Math|Transform|MakeTransform (.ImpactPoint (Collision|BreakHitResult _outhit)) "0, 0, 0" "1.000000,1.000000,1.000000") "Undefined" "MultiplyWithRoot" 0 0)))))

(event EventBeginPlay
  (|CallParentFunction))

(event EventOnExplosionEffects
  (params (HitActor :type Actor%20Object%20Reference))
  (bind _grenade (Variables|Default|GetGrenade))
  (bind _returnvalue (Transformation|GetWorldLocation _grenade))
  (Utilities|FlowControl|DoOnce false
    (:Completed
      (Class|GameplayStatics|PrimeSound "/Game/ModelTextureArtTest/IceGrenade/FireGrenade_SFX_Cue.FireGrenade_SFX_Cue")
      (Audio|PlaySound2D "/Game/ModelTextureArtTest/IceGrenade/FireGrenade_SFX_Cue.FireGrenade_SFX_Cue" 1.0 1.0 0.0 0 0)
      (bind _outhit (Collision|LineTraceByChannel (+ _returnvalue "0.000000,0.000000,1000.000000") (- _returnvalue "0.000000,0.000000,20000.000000") "TraceTypeQuery1" true 0 "None"))
      (if (.bBlockingHit (Collision|BreakHitResult _outhit))
        (Game|SpawnActorfromClass "/Game/Blueprints/Grenades/BP_HazardFire.BP_HazardFire_C" (Math|Transform|MakeTransform (.ImpactPoint (Collision|BreakHitResult _outhit)) "0, 0, 0" "1.000000,1.000000,1.000000") "Undefined" "MultiplyWithRoot" 0 0)))))

(fn ConstructionScript
  (|CallParentFunction))