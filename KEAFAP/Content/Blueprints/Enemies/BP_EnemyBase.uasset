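; Base enemy character that reads its stats from DT_EnemyStats by row name and registers with the level's BP_WaveManager.
; It provides montage-notify melee attacks, projectile firing and a shot cooldown.
; Point damage to the mesh doubles on headshots, spawns Niagara blood and sends hit feedback, with score and clock rewards on kills.
; Status effects attach as runtime components, and an action speed multiplier scales walk speed and shot cooldown.
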(event EventBeginPlay
  (Utilities|FlowControl|Sequence
    (:then_0
      ;[0.15 0.15 0.15 0.5] Assign Enemy Stats
      (bind _returnvalue (Utilities|GetDataTableRow "/Game/Data/DT_EnemyStats.DT_EnemyStats" (Variables|Default|GetEnemyStatsRowName))
        (:then
          (bind _output_get (Variables|Stats|SetMaxHealth (.Health (Utilities|Struct|BreakF_EnemyStats _returnvalue))))
          (Variables|Stats|SetCurrentHealth _output_get)
          (Variables|/Script/Engine.CharacterMovementComponent|SetMaxAcceleration (Variables|Character|GetCharacterMovement) (.MoveSpeed (Utilities|Struct|BreakF_EnemyStats _returnvalue))))
        (:RowNotFound
          (Development|PrintString (Utilities|String|Append "ERROR: " (Utilities|GetClassDisplayName (Utilities|GetClass self)) " does not have a valid Data Table Row Name!") true true "(R=1.000000,G=0.017564,B=0.000000,A=1.000000)"))))
    (:then_1
      ;[0.15 0.15 0.15 0.5] Report self to Wave Manager
      (bind _returnvalue_2 (Actor|GetActorOfClass "/Game/Blueprints/Enemies/BP_WaveManager.BP_WaveManager_C"))
      (Utilities|IsValid _returnvalue_2
        (:Is%20Valid
          (bind _output_get_2 (Variables|Default|SetWaveManager _returnvalue_2))
          (Default|AddNewEnemy _output_get_2 self))
        (:Is%20Not%20Valid
          (Development|PrintString "WARNING: No wave manager in this level!" true true "(R=1.000000,G=0.915845,B=0.000000,A=1.000000)" 2.0 "WM_Warning"))))))

(event EventAttack
  ;[0.15 0.15 0.15 0.5] Event Attack
  (Animation|Montage|PlayMontage (Variables|Character|GetMesh) "/Game/AI/Animations/MNTG_Attack.MNTG_Attack"
    (:OnCompleted
      (Default|CallOnAttackEnd :!label _label))
    (:OnInterrupted
      (goto _label))
    (:OnNotifyBegin
      ;;[0.15 0.15 0.15 0.5] Deal Damage to Player if within range
      (bind _returnvalue (Utilities|GetDataTableRow "/Game/Data/DT_EnemyStats.DT_EnemyStats" (Variables|Default|GetEnemyStatsRowName))
        (:then
          (if (>= (.MeleeRange (Utilities|Struct|BreakF_EnemyStats _returnvalue)) (Transformation|GetDistanceTo (Game|GetPlayerCharacter 0)))
            (Game|Damage|ApplyDamage (Game|GetPlayerCharacter 0) (.MeleeDamage (Utilities|Struct|BreakF_EnemyStats _returnvalue)) (AI|GetAIController 0) self)))))))

(event EventFireProjectile
  (params (Attack%20Target :type Actor%20Object%20Reference))
  (bind _firingpoint (Variables|Default|GetFiringPoint))
  (bind _returnvalue (Transformation|GetWorldLocation _firingpoint))
  ;[0.15 0.15 0.15 0.5] Fire Projectile
  (bind _returnvalue_2 (Game|SpawnActorfromClass "/Game/Blueprints/Enemies/BP_Projectile.BP_Projectile_C" (Math|Transform|MakeTransform _returnvalue (Math|Rotator|FindLookatRotation _returnvalue (Transformation|GetActorLocation Attack%20Target)) "1.000000,1.000000,1.000000") "Undefined" "MultiplyWithRoot" 0 self))
  (Utilities|IsValid _returnvalue_2
    (:Is%20Valid
      (Variables|/Game/Blueprints/Enemies/BP_Projectile.BP_Projectile_C|SetEnemyStatsRowName _returnvalue_2 (Variables|Default|GetEnemyStatsRowName)))
    (:Is%20Not%20Valid
      _))
  (Default|CallOnAttackEnd))

(event EventApplyStatusEffect
  (params (Effect%20Class :type AC%20Status%20Effect%20Base%20Class%20Reference) (Duration :type Float%20%28double-precision%29) (Param :type Float%20%28double-precision%29))
  (bind _self self)
  (bind _returnvalue (AI|GetAIController _self))
  ;[0.15 0.15 0.15 0.5] Apply Status Effect
  (Utilities|IsValid _returnvalue
    (:Is%20Valid
      (bind _asaic_enemy_base (Utilities|Casting|CastToAIC_EnemyBase _returnvalue))
      (Game|AddComponentbyClass Effect%20Class Duration Param self _asaic_enemy_base))))

(event EventTick
  (params (DeltaSeconds :type Float%20%28single-precision%29))
  ;[0.15 0.15 0.15 0.5] Reduce Shot Cooldown
  (if (> (Variables|Stats|GetShotCooldown) 0.0)
    (Variables|Stats|SetShotCooldown (- (Variables|Stats|GetShotCooldown) DeltaSeconds))))

(event Game|Damage|EventPointDamage
  (params (Damage :type Float%20%28single-precision%29) (DamageType :type Damage%20Type%20Object%20Reference) (HitLocation :type Vector :default "0, 0, 0") (HitNormal :type Vector :default "0, 0, 0") (HitComponent :type Primitive%20Component%20Object%20Reference) (BoneName :type Name :default "None") (ShotFromDirection :type Vector :default "0, 0, 0") (InstigatedBy :type Controller%20Object%20Reference) (DamageCauser :type Actor%20Object%20Reference) (HitInfo :type Hit%20Result%20Structure%20%28by%20ref%29))
  (bind _impactpoint (Collision|BreakHitResult HitInfo))
  (bind _returnvalue (== BoneName "head"))
  (bind _currenthealth (Variables|Stats|GetCurrentHealth))
  (bind _returnvalue_2 (<= _currenthealth 0.0))
  ;[0.15 0.15 0.15 0.5] Take Point Damage
  (if (== HitComponent (Variables|Character|GetMesh))
    (if _returnvalue
      (CallFunction|ReduceHealth (* Damage 2.0) false false)
      (CallFunction|EmitBloodBurst _impactpoint 3 10 8.0 12.0 1e+03)
      (else
        (CallFunction|ReduceHealth Damage false false)
        (CallFunction|EmitBloodBurst _impactpoint 3 3 4.0 8.0 3.5e+02)))
    (Utilities|FlowControl|Sequence
      (:then_0
        (if _returnvalue_2
          ;[0.15 0.15 0.15 0.5] Kill Enemy
          (CallFunction|EmitBloodBurst (Transformation|GetActorLocation) 10 5 12.0 16.0 1.5e+03)
          (Actor|DestroyActor)
          (bind _returnvalue_3 (Utilities|GetDataTableRow "/Game/Data/DT_EnemyStats.DT_EnemyStats" (Variables|Default|GetEnemyStatsRowName))
            (:then
              (Class|BPIGameState|AddTimetoClock(Message) (Game|GetGameState) 1000)
              (Class|BPIInteract|AddScore(Message) (Game|GetPlayerCharacter 0) (Math|Float|Truncate (.EXP (Utilities|Struct|BreakF_EnemyStats _returnvalue_3))))))))
      (:then_1
        (Class|BPIInteract|AddHit(Message) (Game|GetPlayerCharacter 0) _returnvalue _returnvalue_2)))))

(fn ConstructionScript)

(fn ReduceHealth
  (params (Amount :type Float%20%28double-precision%29) (Print%20Health :type Boolean) (Print%20Damage :type Boolean))
  (bind _wavemanager (Variables|Default|GetWaveManager))
  (Variables|Stats|SetCurrentHealth (- (Variables|Stats|GetCurrentHealth) Amount))
  (Utilities|FlowControl|Sequence
    (:then_0
      ;[0.15 0.15 0.15 0.5] Print Resulting Health
      (if Print%20Health
        (Development|PrintString (Utilities|String|Append "Current Health: " (Utilities|String|ToString(Float) (Variables|Stats|GetCurrentHealth)) "/" (Utilities|String|ToString(Float) (Variables|Stats|GetMaxHealth))) true true "(R=0.000000,G=1.000000,B=0.050767,A=1.000000)")))
    (:then_1
      ;[0.15 0.15 0.15 0.5] Print Damage Taken
      (if Print%20Damage
        (Development|PrintString (Utilities|String|Append (Utilities|GetDisplayName self) " took " (Utilities|String|ToString(Float) Amount) " damage!") true true "(R=1.000000,G=0.000000,B=0.018814,A=1.000000)")))
    (:then_2
      ;[0.15 0.15 0.15 0.5] If Health < 0
      (if (<= (Variables|Stats|GetCurrentHealth) 0.0)
        (Utilities|IsValid _wavemanager
          (:Is%20Valid
            (Default|RemoveEnemy _wavemanager self))
          (:Is%20Not%20Valid
            _))
        (Actor|DestroyActor)))))

(fn SetActionSpeed
  (params (New%20Speed :type Float%20%28double-precision%29))
  (bind _charactermovement (Variables|Character|GetCharacterMovement))
  (LocalVariables|SetOld%20Speed (Variables|Stats|GetActionSpeedMultiplier))
  (LocalVariables|SetSpeed%20Change%20Factor (/ New%20Speed (LocalVariables|GetOld%20Speed)))
  (Variables|Stats|SetActionSpeedMultiplier New%20Speed)
  (Variables|/Script/Engine.CharacterMovementComponent|SetMaxWalkSpeed _charactermovement (* (LocalVariables|GetSpeed%20Change%20Factor) (Variables|/Script/Engine.CharacterMovementComponent|GetMaxWalkSpeed _charactermovement)))
  (Variables|Stats|SetShotCooldown (/ (Variables|Stats|GetShotCooldown) (LocalVariables|GetSpeed%20Change%20Factor))))

(fn ResetActionSpeed
  (CallFunction|SetActionSpeed 1.0))

(fn ResetShotCooldown
  (bind _returnvalue (Utilities|GetDataTableRow "/Game/Data/DT_EnemyStats.DT_EnemyStats" (Variables|Default|GetEnemyStatsRowName))
    (:then
      (Variables|Stats|SetShotCooldown (/ (/ 1.0 (.FireRate (Utilities|Struct|BreakF_EnemyStats _returnvalue))) (Variables|Stats|GetActionSpeedMultiplier))))))

(fn EmitBloodBurst
  (params (Location :type Vector) (Loops :type Integer) (Count :type Integer) (SizeMin :type Float%20%28double-precision%29) (SizeMax :type Float%20%28double-precision%29) (InitialVelocity :type Float%20%28double-precision%29))
  (for _index (range 1 Loops)
    (bind _returnvalue (Niagara|SpawnSystematLocation "/Game/Particles/NS_BloodBurst.NS_BloodBurst" Location "0, 0, 0" (Math|Conversions|ToVector(Float) 0.5) true false "AutoRelease"))
    (Class|NiagaraComponent|SetVariableInt _returnvalue "User.Count" Count)
    (Niagara|SetNiagaraVariable(Float) _returnvalue "User.Size" (Math|Random|RandomFloatinRange SizeMin SizeMax))
    (Niagara|SetNiagaraVariable(LinearColor) _returnvalue "User.BloodColor" (Utilities|Struct|MakeLinearColor (Math|Random|RandomFloatinRange 0.3 0.8) 0.0 0.0 1.0))
    (Niagara|SetNiagaraVariable(Float) _returnvalue "User.InitialVelocity" InitialVelocity)
    (Components|Activation|Activate _returnvalue false)))

(fn SetMovementSpeed
  (params (Speed :type E_MovementSpeed%20Enum :default "NewEnumerator0"))
  (bind _returnvalue (Utilities|GetDataTableRow "/Game/Data/DT_EnemyStats.DT_EnemyStats" (Variables|Default|GetEnemyStatsRowName))
    (:then
      (bind _output_get (Variables|/Script/Engine.CharacterMovementComponent|SetMaxWalkSpeed (Variables|Character|GetCharacterMovement) (Utilities|Select :Index Speed :NewEnumerator0 (* (Variables|Stats|GetActionSpeedMultiplier) (* (.MoveSpeed (Utilities|Struct|BreakF_EnemyStats _returnvalue)) 0.5)) :NewEnumerator1 (* (.MoveSpeed (Utilities|Struct|BreakF_EnemyStats _returnvalue)) (Variables|Stats|GetActionSpeedMultiplier)))))
      (return _output_get))
    (:RowNotFound
      (Development|PrintString "Enemy is missing its row in the data table!"))))