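; BP_HeavyEnemy is a heavy enemy with two attacks: a projectile burst and a ground slam.
; The burst fires timed shots from the firing point at the target's current location, passing the enemy's stats row name to each projectile.
; The slam plays a Niagara effect below the enemy, spawns BP_HeavySlam after a delay and runs on a timer-driven cooldown.
; Both attacks signal their completion through OnAttackEnd.
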(event Custom|Event%20Slam
  (bind _returnvalue (Transformation|GetActorLocation))
  (bind _returnvalue_2 (Math|Float|MakeLiteralFloat 2.0))
  (bind _returnvalue_3 (- _returnvalue "0.000000,0.000000,135.000000"))
  ;[0.15 0.15 0.15 0.5] Slam
  (Variables|SlamAbility|SetSlamReady false)
  (Utilities|Time|SetTimerbyEvent (delegate Custom|OnSlamCDEnd) (Variables|Default|GetSlamCD))
  (Niagara|SpawnSystematLocation "/Game/Particles/NS_Slam.NS_Slam" _returnvalue_3)
  (Utilities|FlowControl|Delay 1.0)
  (Game|SpawnActorfromClass "/Game/Blueprints/Enemies/BP_HeavySlam.BP_HeavySlam_C" (Math|Transform|MakeTransform _returnvalue_3 "0, 0, 0" (Math|Vector|MakeVector _returnvalue_2 _returnvalue_2 1.0)) "Undefined" "MultiplyWithRoot" 0 0)
  (Utilities|FlowControl|Delay 2.0)
  (Default|CallOnAttackEnd))

(event Custom|OnSlamCDEnd
  ;[0.15 0.15 0.15 0.5] Slam
  (Variables|SlamAbility|SetSlamReady true))

(event EventBeginPlay
  (|CallParentFunction) ; This node is disabled and will not be called.\nDrag off pins to build functionality.
)

(event Collision|EventActorBeginOverlap
  (params (OtherActor :type Actor%20Object%20Reference)))

(event EventFireProjectile
  (params (Attack%20Target :type Actor%20Object%20Reference))
  ;[0.15 0.15 0.15 0.5] Fire Projectile Burst
  (Variables|BurstFire|SetBurstIndex (Variables|BurstFire|GetBurstCount))
  (CallFunction|Shoot (Transformation|GetActorLocation Attack%20Target) :!label _label)
  (bind _result (Math|Integer|DecrementInt (Variables|BurstFire|GetBurstIndex))
    (:%20%20
      (if (> _result 0)
        (Utilities|FlowControl|Delay (Variables|BurstFire|GetSplitTime))
        (goto _label)
        (else
          (Default|CallOnAttackEnd))))))

(event EventTick
  (params (DeltaSeconds :type Float%20%28single-precision%29))
  (|CallParentFunction DeltaSeconds) ; This node is disabled and will not be called.\nDrag off pins to build functionality.
)

(fn ConstructionScript
  (|CallParentFunction))

(fn Shoot
  (params (Target :type Vector))
  (bind _firingpoint (Variables|Default|GetFiringPoint))
  (bind _returnvalue (Transformation|GetWorldLocation _firingpoint))
  (bind _returnvalue_2 (Game|SpawnActorfromClass "/Game/Blueprints/Enemies/BP_Projectile.BP_Projectile_C" (Math|Transform|MakeTransform _returnvalue (Math|Rotator|FindLookatRotation _returnvalue Target) "1.000000,1.000000,1.000000") "Undefined" "MultiplyWithRoot" 0 self))
  (Utilities|IsValid _returnvalue_2
    (:Is%20Valid
      (Variables|/Game/Blueprints/Enemies/BP_Projectile.BP_Projectile_C|SetEnemyStatsRowName _returnvalue_2 (Variables|Default|GetEnemyStatsRowName)))))