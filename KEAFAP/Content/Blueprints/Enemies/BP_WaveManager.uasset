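; Wave manager that runs enemy waves, reading light, medium and heavy counts from DT_EnemyWaves and repeating the last row once exhausted.
; WarmupDone gathers spawnpoints and starts the first wave; Tick feeds randomly picked queued enemies to them until the queue empties.
; After spawning, when the count reaches NextWaveThreshold, remaining enemies are destroyed if at most one is visible to the player.
; A zero count fires WaveEnd, starting the next wave.
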(event Custom|WaveEnd_Event
  (Variables|Default|SetState "NewEnumerator2")
  (CallFunction|FStartNextWave))

(event EventBeginPlay
  (Utilities|FlowControl|Sequence
    (:then_0
      (bind _outrownames (DataTable|GetDataTableRowNames "/Game/Data/DT_EnemyWaves.DT_EnemyWaves"))
      (Variables|Default|SetWaveTableRows _outrownames))
    (:then_1
      (Class|BPIGameState|RegisterNewListener(Message) (Game|GetGameState) self)
      (EventDispatchers|BindEventtoWaveEnd (EventDispatchers|CreateEvent :!event Custom|WaveEnd_Event)))))

(event EventWarmupDone
  (Utilities|FlowControl|DelayUntilNextTick)
  (if (<= (Variables|Default|GetEnemyCount) (Variables|Default|GetNextWaveThreshold))
    (CallFunction|RefreshSpawnpoints)
    ;[0.15 0.15 0.15 0.5] This starts the first wave on begin play
    (CallFunction|FStartNextWave)))

(event EventTick
  (params (DeltaSeconds :type Float%20%28single-precision%29))
  (bind _enemiestospawn (Variables|Default|GetEnemiesToSpawn))
  (bind (_outitem _outindex) (Utilities|Array|Random _enemiestospawn))
  (Utilities|FlowControl|Sequence
    (:then_0
      ;[0.15 0.15 0.15 0.5] DEBUG: Show Enemy Count
      (if (Variables|Debug|GetDisplayEnemyCount)
        (Development|PrintString (Utilities|String|Append "Enemies Alive: " (Utilities|String|ToString(Integer) (Variables|Default|GetEnemyCount))) true true "(R=0.839079,G=0.257579,B=1.000000,A=1.000000)" 2.0 "Enemy Count")))
    (:then_1
      ;[0.15 0.15 0.15 0.5] Spawn Enemies if Needed
      (if (Utilities|Enum|Equal(Enum) (Variables|Default|GetState) "NewEnumerator0")
        (if (not (Utilities|Array|IsEmpty (Variables|Default|GetEnemiesToSpawn)))
          (bind _array_element (Utilities|Array|ForEachLoopwithBreak (Variables|Default|GetSpawnPoints) :!label _label)
            (:LoopBody
              (bind _spawnedenemy (Default|SpawnEnemy _array_element _outitem))
              (if _spawnedenemy
                (Utilities|Array|RemoveIndex (Variables|Default|GetEnemiesToSpawn) _outindex))
              (if (Utilities|Array|IsEmpty (Variables|Default|GetEnemiesToSpawn))
                (goto _label Break)))
            (:Completed
              ;[0.15 0.15 0.15 0.5] After each spawning loop, check if we are done spawning
              (if (Utilities|Array|IsEmpty (Variables|Default|GetEnemiesToSpawn))
                (Variables|Default|SetState "NewEnumerator1")
                ;[0.15 0.15 0.15 0.5] When finished, check if we need to start next wave
                (CallFunction|WaveEndCheck)))))))))

(event EventStartNextWave
  ;[0.15 0.15 0.15 0.5] Call this when we're good to start spawning
  (CallFunction|FStartNextWave))

(fn ConstructionScript)

(fn AddNewEnemy
  (params (NewEnemy :type BP%20Enemy%20Base%20Object%20Reference))
  (Math|Integer|IncrementInt (Variables|Default|GetEnemyCount)))

(fn RemoveEnemy
  (params (EnemyToRemove :type BP%20Enemy%20Base%20Object%20Reference))
  (Math|Integer|DecrementInt (Variables|Default|GetEnemyCount)
    (:%20%20
      (CallFunction|WaveEndCheck))))

(fn FStartNextWave
  (bind _wavetablerows (Variables|Default|GetWaveTableRows))
  (bind _result (Math|Integer|IncrementInt (Variables|Default|GetWaveIndex))
    (:%20%20
      (if (Utilities|Array|IsValidIndex _wavetablerows _result)
        _
        (else
          (Variables|Default|SetWaveIndex (Utilities|Array|LastIndex _wavetablerows))))
      (if (Utilities|Array|IsEmpty (Variables|Default|GetSpawnPoints))
        (Development|PrintString "ERROR: Wave Manager has no Spawn Points to use! Spawning Failed" true true "(R=1.000000,G=0.000000,B=0.024422,A=1.000000)")
        (else
          (bind _returnvalue (Utilities|GetDataTableRow "/Game/Data/DT_EnemyWaves.DT_EnemyWaves" (Utilities|Array|Get(acopy) (Variables|Default|GetWaveTableRows) (Variables|Default|GetWaveIndex)))
            (:then
              (Variables|Default|SetState "NewEnumerator0")
              (Utilities|FlowControl|Sequence
                (:then_0
                  (CallFunction|AddEnemiestoSpawn (.Light (Utilities|Struct|BreakF_WaveEnemyCounts _returnvalue)) "/Game/Blueprints/Enemies/BP_LightEnemy.BP_LightEnemy_C"))
                (:then_1
                  (CallFunction|AddEnemiestoSpawn (.Medium (Utilities|Struct|BreakF_WaveEnemyCounts _returnvalue)) "/Game/Blueprints/Enemies/BP_MediumEnemy.BP_MediumEnemy_C"))
                (:then_2
                  (CallFunction|AddEnemiestoSpawn (.Heavy (Utilities|Struct|BreakF_WaveEnemyCounts _returnvalue)) "/Game/Blueprints/Enemies/BP_HeavyEnemy.BP_HeavyEnemy_C"))))
            (:RowNotFound
              (Development|PrintString (Utilities|String|Append "ERROR: Invalid DT_EnemyWaves Row! Index: " (Utilities|String|ToString(Integer) (Variables|Default|GetWaveIndex))) true true "(R=1.000000,G=0.034106,B=0.000000,A=1.000000)"))))))))

(fn RefreshSpawnpoints
  (bind _outactors (Actor|GetAllActorsOfClass "/Game/Blueprints/Enemies/BP_EnemySpawnpoint.BP_EnemySpawnpoint_C"))
  (Variables|Default|SetSpawnPoints _outactors))

(fn AddEnemiestoSpawn
  (params (Amount :type Integer) (Enemy :type BP%20Enemy%20Base%20Soft%20Class%20Reference))
  (for _index (range 1 Amount)
    (Utilities|Array|Add (Variables|Default|GetEnemiesToSpawn) Enemy)))

(fn WaveEndCheck
  (bind _returnvalue (Viewport|GetViewportSize))
  (if (and (<= (Variables|Default|GetEnemyCount) (Variables|Default|GetNextWaveThreshold)) (Utilities|Enum|Equal(Enum) (Variables|Default|GetState) "NewEnumerator1"))
    (Utilities|FlowControl|Sequence
      (:then_0
        (LocalVariables|SetEnemiesOnScreen 0)
        (bind _outactors (Actor|GetAllActorsOfClass "/Game/Blueprints/Enemies/BP_EnemyBase.BP_EnemyBase_C"))
        (for _array_element _outactors
          (if (Math|Boolean|ANDBoolean (> (.x (.ScreenLocation (Class|PlayerController|ProjectWorldLocationtoScreen (Game|GetPlayerController (Game|GetPlayerState 0)) (Transformation|GetWorldLocation (Variables|/Script/Engine.Actor|GetRootComponent _array_element)) false))) 0.0) (> (.y (.ScreenLocation (Class|PlayerController|ProjectWorldLocationtoScreen (Game|GetPlayerController (Game|GetPlayerState 0)) (Transformation|GetWorldLocation (Variables|/Script/Engine.Actor|GetRootComponent _array_element)) false))) 0.0) (< (.x (.ScreenLocation (Class|PlayerController|ProjectWorldLocationtoScreen (Game|GetPlayerController (Game|GetPlayerState 0)) (Transformation|GetWorldLocation (Variables|/Script/Engine.Actor|GetRootComponent _array_element)) false))) (.x _returnvalue)) (< (.y (.ScreenLocation (Class|PlayerController|ProjectWorldLocationtoScreen (Game|GetPlayerController (Game|GetPlayerState 0)) (Transformation|GetWorldLocation (Variables|/Script/Engine.Actor|GetRootComponent _array_element)) false))) (.y _returnvalue)) (Controller|LineOfSightTo (Game|GetPlayerController (Game|GetPlayerState 0)) _array_element "0, 0, 0" false))
            (Math|Integer|IncrementInt (LocalVariables|GetEnemiesOnScreen))))
        ;[0.15 0.15 0.15 0.5] If they're all off screen, kill all and skip to next wave
        (if (<= (LocalVariables|GetEnemiesOnScreen) 1)
          (for _array_element_2 _outactors
            (Actor|DestroyActor _array_element_2))
          (Variables|Default|SetEnemyCount 0)))
      (:then_1
        (if (== (Variables|Default|GetEnemyCount) 0)
          (Variables|Default|SetState "NewEnumerator2")
          (Default|CallWaveEnd))))))

(fn GetRemainingTime
  (return 0))