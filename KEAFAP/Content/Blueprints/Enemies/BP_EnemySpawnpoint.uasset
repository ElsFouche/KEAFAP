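; BP_EnemySpawnpoint is an enemy spawn point that spawns a requested enemy class within a radius around itself.
; SpawnEnemy succeeds only when the point is ready and the class is in EnemyList, returning whether it spawned.
; Spawns use a random angle and distance, then start a randomized cooldown timer before the point is ready again.
; The construction script draws a debug cylinder showing the spawn radius.
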(event Custom|OnSpawnCDEnd
  (Variables|Default|SetReadyToSpawn true))

(fn ConstructionScript
  (bind _returnvalue (Transformation|GetActorLocation))
  (Class|KismetSystemLibrary|DrawDebugCylinder _returnvalue (+ _returnvalue "0.000000,0.000000,10.000000") (Variables|Default|GetSpawnRadius) 12 "(R=0.000000,G=1.000000,B=0.049294,A=1.000000)" 0.0 0.0))

(fn SpawnEnemy
  (params (Enemy :type BP%20Enemy%20Base%20Soft%20Class%20Reference))
  (LocalVariables|SetRequestedEnemy (Utilities|ResolveSoftReference Enemy))
  (if (Variables|Default|GetReadyToSpawn)
    (if (Utilities|Array|ContainsItem (Variables|Default|GetEnemyList) (LocalVariables|GetRequestedEnemy))
      (Game|SpawnActorfromClass (LocalVariables|GetRequestedEnemy) (Math|Transform|MakeTransform (+ (Transformation|GetActorLocation) (Math|Vector|RotateVectorAroundAxis (Math|Vector|MakeVector (Math|Random|RandomFloatinRange 0.0 (Variables|Default|GetSpawnRadius)) 0.0 0.0) (Math|Random|RandomFloatinRange 0.0 3.6e+02) "0.000000,0.000000,1.000000")) "0, 0, 0" "1.000000,1.000000,1.000000") "AdjustIfPossibleButAlwaysSpawn" "MultiplyWithRoot" 0 0)
      (Utilities|Time|SetTimerbyEvent (EventDispatchers|CreateEvent :!event Custom|OnSpawnCDEnd) (Math|Random|RandomFloatinRange (Variables|Default|GetSpawnCooldownMin) (Variables|Default|GetSpawnCooldownMax)))
      (Variables|Default|SetReadyToSpawn false)
      (return true)
      (else
        _)))
  (return false))