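; BP_Projectile is an enemy projectile that damages whatever actor its collider hits.
; On BeginPlay it sets a ten-second lifespan and reads its row from DT_EnemyStats, writing the projectile speed to the movement component's InitialSpeed.
; Hits apply that row's projectile damage and print the amount, without destroying the projectile.
; A missing row only prints an error.
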(event OnComponentHit(Collider)
  (params (HitComponent :type Primitive%20Component%20Object%20Reference) (OtherActor :type Actor%20Object%20Reference) (OtherComp :type Primitive%20Component%20Object%20Reference) (NormalImpulse :type Vector :default "0, 0, 0") (Hit :type Hit%20Result%20Structure%20%28by%20ref%29))
  (bind _returnvalue (Game|Damage|ApplyDamage OtherActor (.ProjectileDamage (Utilities|Struct|BreakF_EnemyStats (stale EventBeginPlay _returnvalue))) 0 0))
  (Development|PrintString (Utilities|String|Append "Dealt " (Utilities|String|ToString(Float) _returnvalue) " damage!")))

(event EventBeginPlay
  (Actor|SetLifeSpan 1e+01)
  (bind _returnvalue (Utilities|GetDataTableRow "/Game/Data/DT_EnemyStats.DT_EnemyStats" (Variables|Default|GetEnemyStatsRowName))
    (:then
      (Variables|/Script/Engine.ProjectileMovementComponent|SetInitialSpeed (Variables|Default|GetProjectileMovement) (.ProjectileSpeed (Utilities|Struct|BreakF_EnemyStats _returnvalue))))
    (:RowNotFound
      (Development|PrintString (Utilities|String|Append "Projectile: No data table row named " (Utilities|String|ToString(Name) (Variables|Default|GetEnemyStatsRowName))) true true "(R=1.000000,G=0.000233,B=0.028704,A=1.000000)"))))

(fn ConstructionScript)