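; BP_HeavySlam is a short-lived enemy slam damage area that hurts the player inside its collision cylinder and destroys itself after a fixed lifetime.
; A tick after spawning it deals initial damage to an overlapping player, while a timer schedules DoDamageCheck.
; DoDamageCheck deals periodic damage and reschedules itself while the player stays inside, otherwise re-arming CanDamagePlayer.
; When armed, entering the cylinder deals immediate tick damage and restarts the timer if inactive.
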(event OnComponentBeginOverlap(CollisionCylinder)
  (params (OverlappedComponent :type Primitive%20Component%20Object%20Reference) (OtherActor :type Actor%20Object%20Reference) (OtherComp :type Primitive%20Component%20Object%20Reference) (OtherBodyIndex :type Integer) (bFromSweep :type Boolean) (SweepResult :type Hit%20Result%20Structure%20%28by%20ref%29))
  (bind _returnvalue (Game|GetPlayerCharacter 0))
  (if (and (== OtherActor _returnvalue) (Variables|Default|GetCanDamagePlayer))
    (Game|Damage|ApplyDamage _returnvalue (Variables|Default|GetDamageTickAmount) 0 self)
    (Variables|Default|SetCanDamagePlayer false)
    (if (not (Utilities|Time|IsTimerActivebyHandle (Variables|Default|GetDamageTimer)))
      (bind _returnvalue_2 (Utilities|Time|SetTimerbyFunctionName 0 "DoDamageCheck" (Variables|Default|GetDamageTickTime)))
      (Variables|Default|SetDamageTimer _returnvalue_2))))

(event Custom|OnLifetimeEnd
  (Actor|DestroyActor))

(event EventBeginPlay
  (Utilities|Time|SetTimerbyEvent (delegate Custom|OnLifetimeEnd) 5.0)
  (Utilities|FlowControl|Sequence
    (:then_0
      (Utilities|FlowControl|DelayUntilNextTick)
      (if (Utilities|Array|ContainsItem (Collision|GetOverlappingActors (Variables|Default|GetCollision%20Cylinder) 0 :!class /Script/Engine.PrimitiveComponent) (Game|GetPlayerCharacter 0))
        (Game|Damage|ApplyDamage (Game|GetPlayerCharacter 0) (Variables|Default|GetInitialDamage) 0 self)))
    (:then_1
      (bind _returnvalue (Utilities|Time|SetTimerbyFunctionName 0 "DoDamageCheck" (Variables|Default|GetDamageTickTime)))
      (Variables|Default|SetDamageTimer _returnvalue))))

(fn ConstructionScript)

(fn DoDamageCheck
  (if (Utilities|Array|ContainsItem (Collision|GetOverlappingActors (Variables|Default|GetCollision%20Cylinder) 0 :!class /Script/Engine.PrimitiveComponent) (Game|GetPlayerCharacter 0))
    (Game|Damage|ApplyDamage (Game|GetPlayerCharacter 0) (Variables|Default|GetDamageTickAmount) 0 self)
    (Utilities|Time|SetTimerbyFunctionName 0 "DoDamageCheck" (Variables|Default|GetDamageTickTime))
    (Variables|Default|SetCanDamagePlayer false)
    (else
      (Variables|Default|SetCanDamagePlayer true)
      (Utilities|Time|InvalidateTimerHandle (Variables|Default|GetDamageTimer)))))