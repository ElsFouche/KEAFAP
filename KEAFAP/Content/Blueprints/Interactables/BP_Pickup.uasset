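; BP_Pickup is a one-time health, armor or ammo pickup, shown as a sprite and collected when the player overlaps its sphere.
; SetPickupType selects a data asset for the type, which supplies the icon, sounds and amounts, with sprite and sounds async loaded from soft references.
; Collection messages the player, with ammo granting half each weapon's DT_WeaponData maximum, then hides the icon, plays a sound and expires shortly after.
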(event OnComponentBeginOverlap(PickupSphere)
  (params (OverlappedComponent :type Primitive%20Component%20Object%20Reference) (OtherActor :type Actor%20Object%20Reference) (OtherComp :type Primitive%20Component%20Object%20Reference) (OtherBodyIndex :type Integer) (bFromSweep :type Boolean) (SweepResult :type Hit%20Result%20Structure%20%28by%20ref%29))
  (bind _pickupdata (Variables|Pickup|GetPickupData))
  (bind _pickupdata_2 (Variables|Pickup|GetPickupData))
  (bind _pickedupsound (Variables|/Game/Blueprints/Interactables/PDA_Pickup.PDA_Pickup_C|GetPickedUpSound _pickupdata))
  (Class|KismetSystemLibrary|IsObjectOfSoftClass OtherActor "/Game/Blueprints/FirstPerson/BP_Player.BP_Player_C"
    (:True
      (Utilities|FlowControl|DoOnce false
        (:Completed
          (switch Utilities|FlowControl|Switch|SwitchonE_PickupType (Variables|/Game/Blueprints/Interactables/PDA_Pickup.PDA_Pickup_C|GetPickupType _pickupdata_2)
            (:NewEnumerator0
              (Class|BPIInteract|AddHealth(Message) OtherActor (Variables|/Game/Blueprints/Interactables/PDA_Pickup.PDA_Pickup_C|GetExtraHealth _pickupdata_2))
              (Rendering|SetVisibility (Variables|Default|GetPickupIcon) false false :!label _label)
              (Utilities|AsyncLoadAsset _pickedupsound
                (:then
                  (Actor|SetLifeSpan 3.0))
                (:Completed
                  (Audio|PlaySoundatLocation (Utilities|ResolveSoftReference _pickedupsound) (Transformation|GetWorldLocation (Variables|Default|GetPickupIcon)) "0, 0, 0" 1.0 1.0 0.0 0 0 0 0))))
            (:NewEnumerator1
              (Class|BPIInteract|AddArmor(Message) OtherActor (Variables|/Game/Blueprints/Interactables/PDA_Pickup.PDA_Pickup_C|GetExtraArmor _pickupdata_2))
              (goto _label))
            (:NewEnumerator2
              (bind _enumvalue (|ForEachE_Weapons)
                (:LoopBody
                  (bind _returnvalue (Utilities|GetDataTableRow "/Game/Data/DT_WeaponData.DT_WeaponData" (Utilities|String|StringToName (Utilities|String|EnumtoString _enumvalue)))
                    (:then
                      (Class|BPIInteract|AddAmmo(Message) OtherActor _enumvalue (/ (Utilities|Struct|BreakF_WeaponStats _returnvalue) 2)))))
                (:then
                  (goto _label))))))))))

(event Custom|SetPickupType
  (params (PickupType :type E_PickupType%20Enum :default "NewEnumerator0"))
  (bind _pickupicon (Variables|Default|GetPickupIcon))
  (bind _output_get (Variables|Pickup|SetPickupData (Utilities|Select :Index PickupType :NewEnumerator0 "/Game/Blueprints/Interactables/DA_HealthPickup.DA_HealthPickup" :NewEnumerator1 "/Game/Blueprints/Interactables/DA_ArmorPickup.DA_ArmorPickup" :NewEnumerator2 "/Game/Blueprints/Interactables/DA_AmmoPickup.DA_AmmoPickup")))
  (Utilities|AsyncLoadAsset (Variables|/Game/Blueprints/Interactables/PDA_Pickup.PDA_Pickup_C|GetSprite _output_get)
    (:Completed
      (Rendering|Components|Sprite|SetSprite _pickupicon (Utilities|ResolveSoftReference (Variables|/Game/Blueprints/Interactables/PDA_Pickup.PDA_Pickup_C|GetSprite _output_get)))
      (Variables|/Script/Engine.BillboardComponent|SetbIsScreenSizeScaled _pickupicon (Variables|/Game/Blueprints/Interactables/PDA_Pickup.PDA_Pickup_C|GetbIsScreenSizeScaled _output_get))
      (Variables|/Script/Engine.BillboardComponent|SetScreenSize _pickupicon (Variables|/Game/Blueprints/Interactables/PDA_Pickup.PDA_Pickup_C|GetSpriteScreenSize _output_get)))))

(event Custom|OnSpawned
  (bind _pickupdata (Variables|Pickup|GetPickupData))
  (bind _spawnsound (Variables|/Game/Blueprints/Interactables/PDA_Pickup.PDA_Pickup_C|GetSpawnSound _pickupdata))
  (Utilities|AsyncLoadAsset _spawnsound
    (:Completed
      (Audio|PlaySoundatLocation (Utilities|ResolveSoftReference _spawnsound) (Transformation|GetWorldLocation (Variables|Default|GetDefaultSceneRoot)) "0, 0, 0" 1.0 1.0 0.0 0 0 0 0))))

(fn ConstructionScript
  (Components|Sphere|SetSphereRadius (Variables|Default|GetPickupSphere) (Variables|Pickup|GetPickupRadius) true))