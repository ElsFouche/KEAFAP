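; BP_FleshCrate is a destructible crate that bursts into blood when its health runs out and can drop a pickup.
; A looping SquashStretch timeline makes the mesh pulse, starting at a random point and re-rolling play rate and scale limits on each reversal.
; Damage drains health; on death it optionally spawns a typed BP_Pickup at an offset location, plays a Niagara burst and destroys itself.
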(event Custom|AnimLoop
  (bind _squashstretch (Variables|Default|GetSquashStretch))
  (Utilities|FlowControl|DoOnce false
    (:Completed
      (Components|Timeline|SetPlaybackPosition (Variables|Default|GetSquashStretch) (Math|Random|RandomFloatinRange 0.0 0.9) false true)
      (bind _alpha (Timeline|SquashStretch Play)
        (:Update
          (Transformation|SetWorldScale3D (Variables|Default|GetSM_FleshCrate) (Math|Interpolation|Ease "EaseInOut" _alpha (Variables|Default|GetSquashMin) (Variables|Default|GetSquashMax) 2.0)))
        (:Finished
          (Components|Timeline|SetPlayRate (Variables|Default|GetSquashStretch) (Math|Random|RandomFloatinRange 0.8 1.3))
          (Utilities|FlowControl|FlipFlop
            (:A
              (Components|Timeline|ReversefromEnd _squashstretch)
              (Variables|Default|SetSquashMin (+ (Math|Vector|MakeVector (Math|Random|RandomFloatinRange 0.7 1.0) (Math|Random|RandomFloatinRange 1.0 1.3) (Math|Random|RandomFloatinRange 0.8 1.0)) (Variables|Interactable|GetScaleOffset))))
            (:B
              (Components|Timeline|PlayfromStart _squashstretch)
              (Variables|Default|SetSquashMax (+ (Math|Vector|MakeVector (Math|Random|RandomFloatinRange 1.0 1.5) (Math|Random|RandomFloatinRange 0.6 1.0) (Math|Random|RandomFloatinRange 1.0 1.3)) (Variables|Interactable|GetScaleOffset))))))))))

(event EventBeginPlay
  (bind _scaleoffset (Variables|Interactable|GetScaleOffset))
  (Variables|Interactable|SetPickupSpawnLocation (Math|Transform|MakeTransform (+ (Transformation|GetActorLocation) (.location (Variables|Interactable|GetPickupSpawnLocation))) (.rotation (Variables|Interactable|GetPickupSpawnLocation)) (.scale (Variables|Interactable|GetPickupSpawnLocation))))
  (Variables|Default|SetSquashMin (+ (Variables|Default|GetSquashMin) _scaleoffset))
  (Variables|Default|SetSquashMax (+ _scaleoffset (Variables|Default|GetSquashMax)))
  (CallFunction|AnimLoop))

(event Game|Damage|EventAnyDamage
  (params (Damage :type Float%20%28single-precision%29) (DamageType :type Damage%20Type%20Object%20Reference) (InstigatedBy :type Controller%20Object%20Reference) (DamageCauser :type Actor%20Object%20Reference))
  (bind _output_get (Variables|Interactable|SetCrateHealth (- (Variables|Interactable|GetCrateHealth) Damage)))
  (if (<= _output_get 0.0)
    (Utilities|FlowControl|DoOnce false
      (:Completed
        (if (Variables|Interactable|GetbSpawnPickup)
          (bind _returnvalue (Game|SpawnActorfromClass "/Game/Blueprints/Interactables/BP_Pickup.BP_Pickup_C" (Variables|Interactable|GetPickupSpawnLocation) "AlwaysSpawn" "MultiplyWithRoot" 0 0))
          (Default|SetPickupType _returnvalue (Variables|Interactable|GetPickupType))
          (Default|OnSpawned _returnvalue))
        (Niagara|SpawnSystematLocation "/Game/Particles/NS_BloodBurst.NS_BloodBurst" (Transformation|GetActorLocation))
        (Actor|DestroyActor)))))

(fn ConstructionScript
  (Transformation|SetWorldScale3D (Variables|Default|GetSM_FleshCrate) (+ (Variables|Interactable|GetScaleOffset) "1.000000,1.000000,1.000000")))