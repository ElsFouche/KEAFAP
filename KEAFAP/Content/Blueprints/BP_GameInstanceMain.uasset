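; Game instance that owns the game's save data object and handles saving, loading and timed autosaving.
; Saves and loads run sync or async, defaulting to an "Autosave" slot; new slots always save synchronously.
; A busy flag skips overlapping saves and gives loads limited delayed retries.
; Loaded data is pushed to every actor implementing BPI_SaveGame, while autosave uses a looping timer.
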(event Custom|Autosave
  ;[0.18 0.3 0.3] Autosave System
  (CallFunction|SaveGame true (Variables|Default|GetSlotName) (Variables|Default|GetUserIndex)))

(event Custom|EnableAutosave
  ;[0.18 0.3 0.3] Autosave System
  (bind _returnvalue (Utilities|Time|SetTimerbyEvent (EventDispatchers|CreateEvent :!event Custom|Autosave) (Variables|Autosave|GetAutosaveTimer) true true))
  (Variables|Autosave|SetAutosaveTimerHandle _returnvalue))

(event Custom|DisableAutosave
  ;[0.18 0.3 0.3] Autosave System
  (Utilities|Time|ClearandInvalidateTimerbyHandle (Variables|Autosave|GetAutosaveTimerHandle)))

(event EventSetAutosaving
  (params (bSetIsEnabled :type Boolean))
  ;[0.18 0.3 0.3] Autosave System
  (if bSetIsEnabled
    (CallFunction|EnableAutosave)
    (else
      (CallFunction|DisableAutosave))))

(event EventSaveGame
  (params (Async :type Boolean) (SlotName :type String) (UserIndex :type Integer))
  ;[0.18 0.3 0.3] Save Game
  (if (not (Variables|Default|GetDiskOpOngoing))
    (Variables|Default|SetUserIndex UserIndex)
    (Utilities|IsEmptyString SlotName
      (:Empty
        (Variables|Default|SetSlotName "Autosave"))
      (:Exists
        (Variables|Default|SetSlotName SlotName)))
    (bind _returnvalue (SaveGame|DoesSaveGameExist (Variables|Default|GetSlotName) (Variables|Default|GetUserIndex)))
    (if _returnvalue
      ;;[0.07 0.28 0.25] Save Game Async / Sync
      (if Async
        (|AsyncSaveGametoSlot (Variables|Default|GetSavedData) (Variables|Default|GetSlotName) (Variables|Default|GetUserIndex)
          (:then
            (Variables|Default|SetDiskOpOngoing true))
          (:Completed
            (Variables|Default|SetDiskOpOngoing false)))
        (else
          (SaveGame|SaveGametoSlot (Variables|Default|GetSavedData) (Variables|Default|GetSlotName) (Variables|Default|GetUserIndex))
          (Variables|Default|SetDiskOpOngoing false)))
      (else
        ;;[0.07 0.28 0.25] New Save Data Initialization
        (bind _output_get (Variables|Default|SetSlotName (Variables|Default|GetSlotName)))
        (bind _output_get_2 (Variables|Default|SetUserIndex (Variables|Default|GetUserIndex)))
        (SaveGame|SaveGametoSlot (Variables|Default|GetSavedData) _output_get _output_get_2)))))

(event EventLoadGame
  (params (Async :type Boolean) (SlotName :type String) (UserIndex :type Integer))
  ;[0.18 0.3 0.3] Load Game
  (if (Variables|Default|GetDiskOpOngoing) :!label _label
    ;;[0.07 0.28 0.25] Load Reattempt
    (Utilities|FlowControl|DoN 3 :!label _label_2
      (:Exit
        (Utilities|FlowControl|Delay 0.2)
        (goto _label)))
    (else
      (Utilities|FlowControl|Sequence
        (:then_0
          (goto _label_2 Reset))
        (:then_1
          (Variables|Default|SetUserIndex UserIndex)
          (Utilities|IsEmptyString SlotName
            (:Empty
              (Variables|Default|SetSlotName "Autosave"))
            (:Exists
              (Variables|Default|SetSlotName SlotName)))
          (bind _returnvalue (SaveGame|DoesSaveGameExist (Variables|Default|GetSlotName) (Variables|Default|GetUserIndex)))
          (if _returnvalue
            ;;[0.07 0.28 0.25] Load Game Async / Sync
            (if Async
              (bind _savegame (|AsyncLoadGamefromSlot (Variables|Default|GetSlotName) (Variables|Default|GetUserIndex))
                (:then
                  (Variables|Default|SetDiskOpOngoing true))
                (:Completed
                  (bind _asbp_save_game_data (Utilities|Casting|CastToBP_SaveGameData _savegame))
                  (CallFunction|LoadAllGameData _asbp_save_game_data)
                  (Variables|Default|SetSavedData _asbp_save_game_data)
                  (Variables|Default|SetDiskOpOngoing false)))
              (else
                (bind _returnvalue_2 (SaveGame|LoadGamefromSlot (Variables|Default|GetSlotName) (Variables|Default|GetUserIndex)))
                (bind _asbp_save_game_data_2 (Utilities|Casting|CastToBP_SaveGameData _returnvalue_2))
                (CallFunction|LoadAllGameData _asbp_save_game_data_2)
                (Variables|Default|SetSavedData _asbp_save_game_data_2)))
            (else
              (Development|PrintString (Utilities|String|Append (Variables|Default|GetSlotName) " Not Found!")))))))))

(event EventInit
  ;[0.18 0.3 0.3] Init Save Game Object
  (bind _returnvalue (SaveGame|CreateSaveGameObject "/Game/Data/BP_SaveGameData.BP_SaveGameData_C"))
  (Variables|Default|SetSavedData _returnvalue)
  (Variables|Default|SetSlotName "Null")
  (Variables|Default|SetUserIndex -1))

(fn LoadAllGameData
  (params (SaveGame :type BP%20Save%20Game%20Data%20Object%20Reference))
  (bind _outactors (Actor|GetAllActorswithInterface "/Game/Blueprints/Interfaces/BPI_SaveGame.BPI_SaveGame_C"))
  (for _array_element _outactors
    (Class|BPISaveGame|SetGameData(Message) _array_element SaveGame))
  (return))

(fn GetGameData
  (return (Variables|Default|GetSavedData)))