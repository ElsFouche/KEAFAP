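; BPFL_Timer is a Blueprint function library that converts timer values between DateTime, a custom FTime struct and integer milliseconds.
; FTime holds minutes, seconds and milliseconds, and integer division and modulo rebuild it from a millisecond count.
; The DateTime conversions read only the minute, second and millisecond fields, so hours and dates are dropped.
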(fn DateTimeMSMtoInt
  (params (Input :type Date%20Time%20Structure))
  (return (+ (* (.minute Input) 60000) (* (.second Input) 1000) (.millisecond Input))))

(fn FTimetoInt
  (params (_ :type F%20Time%20Structure))
  (return (+ (* (.minutes _) 60000) (* (.seconds _) 1000) (.milliseconds _))))

(fn InttoFTime
  (params (_ :type Integer))
  (bind _returnvalue (Math|Integer|%(Integer) _ 60000))
  (return (Utilities|Struct|MakeF_Time (/ _ 60000) (/ _returnvalue 1000) (Math|Integer|%(Integer) _returnvalue 1000))))

(fn DateTimeMSMtoFTime
  (params (Input :type Date%20Time%20Structure))
  (return (Utilities|Struct|MakeF_Time (.minute Input) (.second Input) (.millisecond Input))))