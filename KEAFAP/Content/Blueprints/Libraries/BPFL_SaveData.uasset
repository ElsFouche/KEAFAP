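; Blueprint function library for reading and unlocking player save data: blood, weapons and weapon upgrades.
; All functions reach the data through the Game Instance's GetGameDataMessage.
; Weapon unlocks are added uniquely to a list, while upgrades are bitmasks per weapon in a map, merged with bitwise OR.
; Nothing here writes to disk, and a leftover upgrade-to-weapon Select node is unused.
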(fn GetCurrBlood
  (bind _savedata (Class|BPISaveGame|GetGameData(Message) (Game|GetGameInstance)))
  (return (Variables|/Game/Data/BP_SaveGameData.BP_SaveGameData_C|GetPlayerBlood _savedata)))

(fn GetUnlockedWeapons
  (bind _savedata (Class|BPISaveGame|GetGameData(Message) (Game|GetGameInstance)))
  (return (Variables|/Game/Data/BP_SaveGameData.BP_SaveGameData_C|GetUnlockedWeapons _savedata)))

(fn GetUnlockedUpgrades
  (bind _savedata (Class|BPISaveGame|GetGameData(Message) (Game|GetGameInstance)))
  (return (Variables|/Game/Data/BP_SaveGameData.BP_SaveGameData_C|GetUpgrades _savedata)))

(fn UnlockWeapon
  (params (NewWeapon :type E_Weapons%20Enum :default "NewEnumerator0"))
  (bind _savedata (SaveData|GetSaveData))
  (bind _unlockedweapons (Variables|/Game/Data/BP_SaveGameData.BP_SaveGameData_C|GetUnlockedWeapons _savedata))
  (Utilities|Array|AddUnique _unlockedweapons NewWeapon)
  (return _unlockedweapons))

(fn UnlockUpgrade
  (params (Weapon :type E_Weapons%20Enum :default "NewEnumerator0") (UpgradeBitmask :type Integer))
  (bind _savedata (SaveData|GetSaveData))
  (bind _upgrades (Variables|/Game/Data/BP_SaveGameData.BP_SaveGameData_C|GetUpgrades _savedata))
  (Utilities|Map|Add _upgrades Weapon (Class|KismetMathLibrary|OrIntInt (.Value (Utilities|Map|Find _upgrades Weapon)) UpgradeBitmask))
  (return _upgrades))

(fn GetSaveData
  (bind _savedata (Class|BPISaveGame|GetGameData(Message) (Game|GetGameInstance)))
  (return _savedata))