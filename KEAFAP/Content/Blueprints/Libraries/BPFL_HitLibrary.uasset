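; BPFL_HitLibrary is a Blueprint function library that removes per-actor duplicates from arrays of hit results.
; UniqueHitsPerActor keeps only the first hit for each actor, tracking the actors already seen in a second array.
; UniqueActorsHit returns just the distinct hit actors, collected with AddUnique.
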(fn UniqueHitsPerActor
  (params (Hits :type Array%20of%20Hit%20Result%20Structures))
  (bind _uniqueactors (LocalVariables|GetUniqueActors))
  (for _array_element Hits
    (if (not (Utilities|Array|ContainsItem _uniqueactors (.HitActor (Collision|BreakHitResult _array_element))))
      (Utilities|Array|Add _uniqueactors (.HitActor (Collision|BreakHitResult _array_element)))
      (Utilities|Array|Add (LocalVariables|GetLUniqueHits) _array_element)))
  (return (LocalVariables|GetLUniqueHits)))

(fn UniqueActorsHit
  (params (Hits :type Array%20of%20Hit%20Result%20Structures))
  (for _array_element Hits
    (Utilities|Array|AddUnique (LocalVariables|GetLUniqueActors) (.HitActor (Collision|BreakHitResult _array_element))))
  (return (LocalVariables|GetLUniqueActors)))