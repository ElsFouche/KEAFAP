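; Utility function library for reordering actor arrays in place and converting enum bytes to bitmasks.
; Three comb sorts shrink their gap by a factor, ordering by ascending squared distance, descending angle, or ascending distance-angle product.
; The plain angle sort compares world position vectors with the reference location, not directions from it.
; Despite its name, the combined sort multiplies rather than averages, so a positive DistanceWeight leaves the order unchanged.
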(fn CombSortActorsbyDist
  (params (Actors :type Array%20of%20Actor%20Object%20References) (ReferenceLocation :type Vector))
  (LocalVariables|SetStep (Utilities|Array|LastIndex Actors))
  (while (>= (LocalVariables|GetStep) 1)
    (while (< (+ (LocalVariables|GetI) (LocalVariables|GetStep)) (Utilities|Array|Length Actors))
      (if (> (Class|KismetMathLibrary|VectorDistanceSquared (Transformation|GetActorLocation (Utilities|Array|Get(acopy) Actors (LocalVariables|GetI))) ReferenceLocation) (Class|KismetMathLibrary|VectorDistanceSquared (Transformation|GetActorLocation (Utilities|Array|Get(acopy) Actors (+ (LocalVariables|GetI) (LocalVariables|GetStep)))) ReferenceLocation))
        (Utilities|Array|Swap Actors (LocalVariables|GetI) (+ (LocalVariables|GetI) (LocalVariables|GetStep))))
      (Math|Integer|IncrementInt (LocalVariables|GetI)))
    (LocalVariables|SetI 0)
    (LocalVariables|SetStep (Math|Float|Truncate (/ (Math|Conversions|ToFloat(Integer) (LocalVariables|GetStep)) (LocalVariables|GetFactor))))))

(fn CombSortActorsbyAngle
  (params (Actors :type Array%20of%20Actor%20Object%20References) (ReferenceLocation :type Vector))
  (LocalVariables|SetStep (Utilities|Array|LastIndex Actors))
  (while (>= (LocalVariables|GetStep) 1)
    (while (< (+ (LocalVariables|GetI) (LocalVariables|GetStep)) (Utilities|Array|Length Actors))
      (if (< (Vector|GetAngleBetween (Transformation|GetActorLocation (Utilities|Array|Get(acopy) Actors (LocalVariables|GetI))) ReferenceLocation) (Vector|GetAngleBetween (Transformation|GetActorLocation (Utilities|Array|Get(acopy) Actors (+ (LocalVariables|GetI) (LocalVariables|GetStep)))) ReferenceLocation))
        (Utilities|Array|Swap Actors (LocalVariables|GetI) (+ (LocalVariables|GetI) (LocalVariables|GetStep))))
      (Math|Integer|IncrementInt (LocalVariables|GetI)))
    (LocalVariables|SetI 0)
    (LocalVariables|SetStep (Math|Float|Truncate (/ (Math|Conversions|ToFloat(Integer) (LocalVariables|GetStep)) (LocalVariables|GetFactor))))))

(fn GetAngleBetween
  (params (V1 :type Vector) (V2 :type Vector))
  (return (Class|KismetMathLibrary|DegAcos (Math|Vector|DotProduct (Math|Vector|Normalize V1) (Math|Vector|Normalize V2)))))

(fn CombSortbyAvgOfDistandAngle
  (params (Actors :type Array%20of%20Actor%20Object%20References) (ReferenceForward :type Vector) (ReferenceLocation :type Vector) (DistanceWeight :type Float%20%28double-precision%29))
  (LocalVariables|SetStep (Utilities|Array|LastIndex Actors))
  (while (>= (LocalVariables|GetStep) 1)
    (while (< (+ (LocalVariables|GetI) (LocalVariables|GetStep)) (Utilities|Array|Length Actors))
      (if (> (* (* (Math|Vector|Distance(Vector) (Transformation|GetActorLocation (Utilities|Array|Get(acopy) Actors (LocalVariables|GetI))) ReferenceLocation) DistanceWeight) (Vector|GetAngleBetween (- (Transformation|GetActorLocation (Utilities|Array|Get(acopy) Actors (LocalVariables|GetI))) ReferenceLocation) ReferenceForward)) (* (Vector|GetAngleBetween (- (Transformation|GetActorLocation (Utilities|Array|Get(acopy) Actors (+ (LocalVariables|GetI) (LocalVariables|GetStep)))) ReferenceLocation) ReferenceForward) (* (Math|Vector|Distance(Vector) (Transformation|GetActorLocation (Utilities|Array|Get(acopy) Actors (+ (LocalVariables|GetI) (LocalVariables|GetStep)))) ReferenceLocation) DistanceWeight)))
        (Utilities|Array|Swap Actors (LocalVariables|GetI) (+ (LocalVariables|GetI) (LocalVariables|GetStep))))
      (Math|Integer|IncrementInt (LocalVariables|GetI)))
    (LocalVariables|SetI 0)
    (LocalVariables|SetStep (Math|Float|Truncate (/ (Math|Conversions|ToFloat(Integer) (LocalVariables|GetStep)) (LocalVariables|GetFactor))))))

(fn EnumtoBitmask
  (params (InByte :type Byte))
  (return (Math|Float|Round (Math|Float|Power 2.0 (Math|Conversions|ToFloat(Byte) InByte)))))