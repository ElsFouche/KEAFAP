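; Base enemy character Blueprint that pulls its stats from DT_EnemyStats by row name.
; BeginPlay sets health and max acceleration from that row, and SetMovementSpeed maps a Walking or Running choice to half or full MoveSpeed.
; Attack plays a montage whose notify checks melee range to the player and only prints damage or distance, then calls OnAttackEnd on completion or interruption.
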(event EventBeginPlay
  (bind _returnvalue (Utilities|GetDataTableRow "/Game/Data/DT_EnemyStats.DT_EnemyStats" (Variables|Default|GetEnemyStatsRowName))
    (:then
      (bind _output_get (Variables|Stats|SetMaxHealth (.Health (Utilities|Struct|BreakF_EnemyStats _returnvalue))))
      (Variables|Stats|SetCurrentHealth _output_get)
      (Variables|/Script/Engine.CharacterMovementComponent|SetMaxAcceleration (Variables|Character|GetCharacterMovement) (.MoveSpeed (Utilities|Struct|BreakF_EnemyStats _returnvalue))))
    (:RowNotFound
      (Development|PrintString "Enemy is missing its row in the data table!"))))

(event EventAttack
  (bind _returnvalue (Game|GetPlayerCharacter 0))
  (bind _returnvalue_2 (Transformation|GetDistanceTo _returnvalue))
  (Animation|Montage|PlayMontage (Variables|Character|GetMesh) "/Game/AI/Animations/MNTG_Attack.MNTG_Attack"
    (:OnCompleted
      (Default|CallOnAttackEnd :!label _label))
    (:OnInterrupted
      (goto _label))
    (:OnNotifyBegin
      ;[0.15 0.15 0.15 0.5] Deal Damage to Player if within range
      (bind _returnvalue_3 (Utilities|GetDataTableRow "/Game/Data/DT_EnemyStats.DT_EnemyStats" (Variables|Default|GetEnemyStatsRowName))
        (:then
          (if (>= (.MeleeRange (Utilities|Struct|BreakF_EnemyStats _returnvalue_3)) _returnvalue_2)
            ;;[0.15 0.15 0.15 0.5] Print the damage dealt
            (Development|PrintString (Utilities|String|Append (Utilities|String|MakeLiteralString "Enemy dealt ") (Utilities|String|ToString(Float) (.MeleeDamage (Utilities|Struct|BreakF_EnemyStats _returnvalue_3))) (Utilities|String|MakeLiteralString " to Player!")))
            (else
              ;;[0.15 0.15 0.15 0.5] Print the distance to the target
              (Development|PrintString (Utilities|String|Append "Distance: " (Utilities|String|ToString(Float) _returnvalue_2))))))))))

(fn ConstructionScript)

(fn SetMovementSpeed
  (params (Speed :type E_MovementSpeed%20Enum :default "NewEnumerator0"))
  (bind _returnvalue (Utilities|GetDataTableRow "/Game/Data/DT_EnemyStats.DT_EnemyStats" (Variables|Default|GetEnemyStatsRowName))
    (:then
      (bind _output_get (Variables|/Script/Engine.CharacterMovementComponent|SetMaxWalkSpeed (Variables|Character|GetCharacterMovement) (Utilities|Select :Index Speed :NewEnumerator0 (* (.MoveSpeed (Utilities|Struct|BreakF_EnemyStats _returnvalue)) 0.5) :NewEnumerator1 (.MoveSpeed (Utilities|Struct|BreakF_EnemyStats _returnvalue)))))
      (return _output_get))
    (:RowNotFound
      (Development|PrintString "Enemy is missing its row in the data table!"))))