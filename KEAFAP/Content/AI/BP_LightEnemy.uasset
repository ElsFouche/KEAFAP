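; BP_LightEnemy is a light enemy Blueprint whose construction script only calls its parent's.
; Its BeginPlay, overlap and Tick events are empty, so this graph adds no live behavior.
; An unconnected debug chain reads health from DT_EnemyStats by row name, then after a delay repeatedly drains and prints it, destroying the actor at zero.
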(event EventBeginPlay)

(event EventTick
  (params (DeltaSeconds :type Float%20%28single-precision%29)))

(event Collision|EventActorBeginOverlap
  (params (OtherActor :type Actor%20Object%20Reference)))

(fn ConstructionScript
  (|CallParentFunction))