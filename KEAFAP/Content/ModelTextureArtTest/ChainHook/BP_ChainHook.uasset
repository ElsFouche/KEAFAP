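; Chain hook projectile that is launched along its local X axis at the speed passed to StartMovement.
; The hook mesh's overlap stops movement, then fires ChainHookHit with the actor and sweep result for enemies or flesh crates; anything else gives the hook a brief lifespan before it disappears.
; The construction script is empty, leaving a disconnected loop meant to build chain links as HISM instances that never runs.
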(event OnComponentBeginOverlap(hook_standalone)
  (params (OverlappedComponent :type Primitive%20Component%20Object%20Reference) (OtherActor :type Actor%20Object%20Reference) (OtherComp :type Primitive%20Component%20Object%20Reference) (OtherBodyIndex :type Integer) (bFromSweep :type Boolean) (SweepResult :type Hit%20Result%20Structure%20%28by%20ref%29))
  (Components|Movement|StopMovementImmediately (Variables|Default|GetProjectileMovement))
  (Class|KismetSystemLibrary|IsObjectOfSoftClass OtherActor "/Game/Blueprints/Enemies/BP_EnemyBase.BP_EnemyBase_C"
    (:True
      (Default|CallChainHookHit OtherActor SweepResult :!label _label))
    (:False
      (Class|KismetSystemLibrary|IsObjectOfSoftClass OtherActor "/Game/Blueprints/Interactables/BP_FleshCrate.BP_FleshCrate_C"
        (:True
          (goto _label))
        (:False
          (Actor|SetLifeSpan 0.2))))))

(fn ConstructionScript)

(fn StartMovement
  (params (Speed :type Float%20%28double-precision%29))
  (Game|Components|ProjectileMovement|SetVelocityinLocalSpace (Variables|Default|GetProjectileMovement) (Math|Vector|MakeVector Speed 0.0 0.0)))