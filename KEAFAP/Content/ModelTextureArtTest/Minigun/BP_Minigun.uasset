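; Minigun actor that visually spins its barrel while the player fires.
; On BeginPlay it binds an event to the minigun spin-up of the player pawn's AC_Shooting component.
; MinigunSpin stores the firing state and, when firing, sets spin speed inversely to the incoming rate.
; Tick rolls BarrelPivot by that speed per frame, unscaled by delta time, and winds it down linearly once firing stops.
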(event Custom|MinigunSpin
  (params (SpinRate :type Float%20%28double-precision%29) (bIsFiring :type Boolean))
  (bind _output_get (Variables|Default|SetbIsFiring bIsFiring))
  (if _output_get
    (Variables|Default|SetSpinRate (Math|Float|SafeDivide 0.5 SpinRate))))

(event EventBeginPlay
  (bind _returnvalue (Game|Player|GetPlayerPawn 0))
  (bind _returnvalue_2 (Actor|GetComponentbyClass _returnvalue "/Game/Blueprints/ActorComponents/AC_Shooting.AC_Shooting_C"))
  (if (and (Utilities|IsValid _returnvalue) (Utilities|IsValid _returnvalue_2))
    (EventDispatchers|BindEventtoMinigunSpinUp _returnvalue_2 (EventDispatchers|CreateEvent :!event Custom|MinigunSpin))))

(event EventTick
  (params (DeltaSeconds :type Float%20%28single-precision%29))
  (if (Variables|Default|GetbIsFiring)
    (Transformation|AddRelativeRotation (Variables|Default|GetBarrelPivot) (Math|Rotator|MakeRotator (Variables|Default|GetSpinRate) 0.0 0.0) false false)
    (elif (> (Variables|Default|GetSpinRate) 0.0)
      (Transformation|AddRelativeRotation (Variables|Default|GetBarrelPivot) (Math|Rotator|MakeRotator (Variables|Default|GetSpinRate) 0.0 0.0) false false)
      (Variables|Default|SetSpinRate (- (Variables|Default|GetSpinRate) (* DeltaSeconds 2e+01))))))

(fn ConstructionScript)